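; Hackable drone pawn that the player flies and fires lasers from, returning control to the StabTemplate character when destroyed by damage or the Abilities input.
; Possession disables gravity, adds damping and shows HackUI; camera-relative forces move the physics body while Tick levels roll.
; Tick also spawns cooldown-limited LaserBolts along camera forward; GetFireRotator's aim-assist sweep is never called.
; InitializeSettings reads invert options but always sets both axis scales to positive.
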(event EventBeginPlay
  (Physics|AddImpulse (Variables|Default|GetPrimaryCollision) (* (Math|Random|RandomUnitVector) 5e+02) "None" true))

(event EventDestroyed
  (if (Variables|Default|GetNoKaboom)
    _
    (else
      (Effects|SpawnEmitteratLocation "/Game/STAB/Particles/Explosion.Explosion" (Transformation|GetActorLocation))))
  (if (not (Utilities|IsValid (Game|Player|GetPlayerPawn 0)))
    (bind _outactors (Actor|GetAllActorsOfClass "/Game/STAB/Blueprints/Abstract/StabTemplate.StabTemplate_C"))
    (Pawn|Possess (Game|GetPlayerController 0) (Utilities|Array|Get(acopy) _outactors))
    (bind _foundwidgets (Widget|GetAllWidgetsOfClass "/Game/STAB/UI/HackUI.HackUI_C" true))
    (for _array_element _foundwidgets
      (Widget|RemovefromParent _array_element))))

(event EventPossessed
  (params (NewController :type Controller%20Object%20Reference))
  (bind _primarycollision (Variables|Default|GetPrimaryCollision))
  (bind _staticmesh (Variables|Default|GetStaticMesh))
  (Utilities|FlowControl|Delay 0.05)
  (if (== (Game|Player|GetPlayerPawn 0) self)
    (Physics|SetEnableGravity _primarycollision false)
    (Class|PrimitiveComponent|SetLinearDamping _primarycollision 5.0)
    (Class|PrimitiveComponent|SetAngularDamping _primarycollision 1e+02)
    (Rendering|Material|SetMaterial _staticmesh 2 "/Game/STAB/Materials/Energy/Laser.Laser")
    (Rendering|Material|SetVectorParameterValueonMaterials _staticmesh "Color" (Variables|Default|GetColor))
    (bind _returnvalue (UserInterface|CreateWidget "/Game/STAB/UI/HackUI.HackUI_C"))
    (UserInterface|Viewport|AddtoPlayerScreen _returnvalue)
    (CallFunction|InitializeSettings)))

(event EventTick
  (params (DeltaSeconds :type Float%20%28single-precision%29))
  (bind _returnvalue (Transformation|GetActorRotation))
  (bind _camera (Variables|Default|GetCamera))
  (bind _speed (Variables|Default|GetSpeed))
  (bind _camera_2 (Variables|Default|GetCamera))
  (bind _downthrusting (Variables|Default|GetDownThrusting))
  (bind _returnvalue_2 (Transformation|GetWorldRotation _camera_2))
  (bind (_roll _pitch _yaw) (Math|Rotator|BreakRotator _returnvalue))
  (bind _returnvalue_3 (Transformation|GetWorldRotation _camera))
  (bind _returnvalue_4 (Math|Vector|GetUpVector _returnvalue_2))
  (bind _returnvalue_5 (* _returnvalue_4 _speed))
  (Utilities|FlowControl|Sequence
    (:then_0
      (if (and (Variables|Default|GetUpThrusting) (not _downthrusting))
        (Physics|AddForce (Variables|Default|GetPrimaryCollision) _returnvalue_5 "None" true)
        (elif _downthrusting
          (Physics|AddForce (Variables|Default|GetPrimaryCollision) (* _returnvalue_5 -1.0) "None" true))))
    (:then_1
      (Variables|Default|SetLifeTimer (+ (Variables|Default|GetLifeTimer) DeltaSeconds))
      (bind _output_get (Variables|Default|SetLaserCooldown (- (Variables|Default|GetLaserCooldown) DeltaSeconds)))
      (if (and (Variables|Default|GetShooting) (<= _output_get 0.0))
        (Variables|Default|SetLaserCooldown 0.15)
        (bind _returnvalue_6 (Game|SpawnActorfromClass "/Game/STAB/Blueprints/Generated/LaserBolt.LaserBolt_C" (Math|Transform|MakeTransform (+ (* (Math|Vector|GetForwardVector _returnvalue_3) 5e+01) (Transformation|GetWorldLocation (Variables|Default|GetStaticMesh))) _returnvalue_3 "1,1,1") "AlwaysSpawn" 0 0))
        (Variables|/Game/STAB/Blueprints/Generated/LaserBolt.LaserBolt_C|SetColor _returnvalue_6 (Variables|Default|GetColor))
        (Variables|/Game/STAB/Blueprints/Generated/LaserBolt.LaserBolt_C|SetShooter _returnvalue_6 self)))
    (:then_2
      (Transformation|SetActorRotation (Math|Interpolation|RInterpTo _returnvalue (Math|Rotator|MakeRotator 0.0 _pitch _yaw) DeltaSeconds 1e+01)))))

(event Game|Damage|EventAnyDamage
  (params (Damage :type Float%20%28single-precision%29) (DamageType :type Damage%20Type%20Object%20Reference) (InstigatedBy :type Controller%20Object%20Reference) (DamageCauser :type Actor%20Object%20Reference))
  (if (> (Variables|Default|GetLifeTimer) 0.5)
    (Actor|DestroyActor)))

(event Input|ActionEvents|InputActionShoot
  (params (Key :type Key%20Structure))
  (:Pressed
    (Variables|Default|SetShooting true))
  (:Released
    (Variables|Default|SetShooting false)))

(event Input|ActionEvents|InputActionJump
  (params (Key :type Key%20Structure))
  (:Pressed
    (Variables|Default|SetUpThrusting true))
  (:Released
    (Variables|Default|SetUpThrusting false)))

(event Input|ActionEvents|InputActionPause
  (params (Key :type Key%20Structure))
  (:Pressed
    (if (Game|IsGamePaused)
      (bind _foundwidgets (Widget|GetAllWidgetsOfClass "/Game/STAB/UI/PausingWidget.PausingWidget_C" false))
      (for _array_element _foundwidgets
        (Default|CloseMenu _array_element))
      (else
        (bind _returnvalue (UserInterface|CreateWidget "/Game/STAB/UI/PauseMenu.PauseMenu_C"))
        (UserInterface|Viewport|AddtoViewport _returnvalue 0)))))

(event Input|ActionEvents|InputActionSlowAim
  (params (Key :type Key%20Structure))
  (bind _springarm (Variables|Default|GetSpringArm))
  (:Pressed
    (Variables|Default|SetTurnSensitivity 12.0)
    (Variables|/Script/Engine.SpringArmComponent|SetTargetArmLength _springarm 1.5e+02))
  (:Released
    (Variables|Default|SetTurnSensitivity 6e+01)
    (Variables|/Script/Engine.SpringArmComponent|SetTargetArmLength _springarm 4e+02)))

(event Input|ActionEvents|InputActionOverdrive
  (params (Key :type Key%20Structure))
  (:Pressed
    (Variables|Default|SetDownThrusting true))
  (:Released
    (Variables|Default|SetDownThrusting false)))

(event Input|ActionEvents|InputActionUse
  (params (Key :type Key%20Structure))
  (bind _camera (Variables|Default|GetCamera))
  (:Pressed
    (bind (_outactors _returnvalue) (Collision|SphereOverlapActors (+ (Transformation|GetWorldLocation _camera) (* (Math|Vector|GetForwardVector _camera) 5e+01)) 1e+02 (Utilities|Array|MakeArray "ObjectTypeQuery1" "ObjectTypeQuery2" "ObjectTypeQuery3" "ObjectTypeQuery4" "ObjectTypeQuery5" "ObjectTypeQuery6") "/Game/STAB/Blueprints/Abstract/Interactable.Interactable_C"))
    (if _returnvalue
      (bind _asinteractable (Utilities|Casting|CastToInteractable (Utilities|Array|Get(acopy) _outactors)))
      (Default|Interact _asinteractable self))))

(event Input|ActionEvents|InputActionAbilities
  (params (Key :type Key%20Structure))
  (:Pressed
    (Actor|DestroyActor)))

(event Input|AxisEvents|InputAxisDroneTurnX
  (params (AxisValue :type Float%20%28single-precision%29))
  (Transformation|AddLocalRotation (Variables|Default|GetPrimaryCollision) (Math|Rotator|MakeRotator 0.0 0.0 (* AxisValue (* (Variables|Default|GetTurnSensitivity) (Utilities|Time|GetWorldDeltaSeconds)) (Variables|Default|GetXScale))) false false))

(event Input|AxisEvents|InputAxisDroneTurnY
  (params (AxisValue :type Float%20%28single-precision%29))
  (Transformation|AddLocalRotation (Variables|Default|GetPrimaryCollision) (Math|Rotator|MakeRotator 0.0 (* AxisValue (* (Variables|Default|GetTurnSensitivity) (Utilities|Time|GetWorldDeltaSeconds)) (Variables|Default|GetYScale)) 0.0) false false))

(event Input|AxisEvents|InputAxisMoveForward
  (params (AxisValue :type Float%20%28single-precision%29))
  (Physics|AddForce (Variables|Default|GetPrimaryCollision) (* (Math|Vector|GetForwardVector (Transformation|GetWorldRotation (Variables|Default|GetCamera))) (* (Variables|Default|GetSpeed) AxisValue)) "None" true))

(event Input|AxisEvents|InputAxisMoveRight
  (params (AxisValue :type Float%20%28single-precision%29))
  (Physics|AddForce (Variables|Default|GetPrimaryCollision) (* (Math|Vector|GetRightVector (Transformation|GetWorldRotation (Variables|Default|GetCamera))) (* (Variables|Default|GetSpeed) AxisValue)) "None" true))

(fn ConstructionScript)

(fn GetFireRotator
  (params (FromLocation :type Vector))
  (bind _array (Utilities|Array|MakeArray "ObjectTypeQuery1" "ObjectTypeQuery2" "ObjectTypeQuery3" "ObjectTypeQuery5" "ObjectTypeQuery6"))
  (bind _camera (Variables|Default|GetCamera))
  (bind _camera_2 (Variables|Default|GetCamera))
  (bind _returnvalue (Transformation|GetWorldLocation _camera))
  (bind _returnvalue_2 (Math|Vector|GetForwardVector _camera))
  (bind _returnvalue_3 (Transformation|GetWorldLocation _camera_2))
  (bind _returnvalue_4 (Math|Vector|GetForwardVector _camera_2))
  (bind _returnvalue_5 (* _returnvalue_2 5.5e+03))
  (bind _returnvalue_6 (+ _returnvalue _returnvalue_5))
  (bind _index (Utilities|FlowControl|ForLoopwithBreak 50 600)
    (:LoopBody
      (bind _returnvalue_7 (Collision|SphereOverlapActors (+ _returnvalue_3 (* _returnvalue_4 (* _index 1e+01))) (+ (* _index 0.2) 2.0) _array 0 (Utilities|Array|MakeArray self)))
      (if _returnvalue_7
        (bind _outhit (Collision|SphereTraceForObjects (+ _returnvalue_3 (* _returnvalue_4 (* _index 9.0))) (+ _returnvalue_3 (* _returnvalue_4 (* _index 11.0))) (+ (* _index 0.2) 2.0) _array false 0 "None"))
        (return (Math|Rotator|FindLookatRotation FromLocation (.impactpoint _outhit)) (.impactpoint _outhit))))
    (:Completed
      (return (Math|Rotator|FindLookatRotation FromLocation _returnvalue_6) _returnvalue_6))))

(fn InitializeSettings
  (bind _asstab_game_instance (Utilities|Casting|CastToStabGameInstance (Game|GetGameInstance)))
  (if (Variables|/Game/STAB/Blueprints/Abstract/StabGameInstance.StabGameInstance_C|GetInvertX _asstab_game_instance)
    _
    (else
      _))
  (Variables|Default|SetXScale 1.0)
  (if (Variables|/Game/STAB/Blueprints/Abstract/StabGameInstance.StabGameInstance_C|GetInvertY _asstab_game_instance)
    _
    (else
      _))
  (Variables|Default|SetYScale 1.0))