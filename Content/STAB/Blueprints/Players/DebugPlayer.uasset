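; DebugPlayer is a player character Blueprint that fires laser pulses and supports an Overdrive boost.
; ClassTick counts down a cooldown while ShootHeld spawns LaserPulse actors just ahead of FirePoint, passing each the player's color and itself as shooter.
; OverdriveToggle switches jump and walk speeds, the flag that shortens fire cooldown, and a color-tinted aura material, with a sound on activation.
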(event EventBeginPlay
  (|CallParentFunction) ; This node is disabled and will not be called.\nDrag off pins to build functionality.
)

(event Collision|EventActorBeginOverlap
  (params (OtherActor :type Actor%20Object%20Reference)))

(event EventTick
  (params (DeltaSeconds :type Float%20%28single-precision%29))
  (|CallParentFunction DeltaSeconds) ; This node is disabled and will not be called.\nDrag off pins to build functionality.
)

(event Game|Damage|EventAnyDamage
  (params (Damage :type Float%20%28single-precision%29) (DamageType :type Damage%20Type%20Object%20Reference) (InstigatedBy :type Controller%20Object%20Reference) (DamageCauser :type Actor%20Object%20Reference)))

(fn ConstructionScript
  (|CallParentFunction))

(fn ClassTick
  (params (DeltaSeconds :type Float%20%28single-precision%29))
  (bind _output_get (Variables|Default|SetLaserCooldown (- (Variables|Default|GetLaserCooldown) DeltaSeconds)))
  (if (and (Variables|Default|GetShootHeld) (<= _output_get 0.0))
    (bind _firerotator (CallFunction|GetFireRotator (Transformation|GetWorldLocation (Variables|Default|GetFirePoint))))
    (if (Variables|Default|GetOverdrive)
      (Variables|Default|SetLaserCooldown 0.1)
      (else
        (Variables|Default|SetLaserCooldown 0.15)))
    (bind _returnvalue (Game|SpawnActorfromClass "/Game/STAB/Blueprints/Generated/LaserPulse.LaserPulse_C" (Math|Transform|MakeTransform (+ (* (Math|Vector|GetForwardVector _firerotator) 5e+01) (Transformation|GetWorldLocation (Variables|Default|GetFirePoint))) _firerotator "1,1,1") "AlwaysSpawn" 0 0))
    (Variables|/Game/STAB/Blueprints/Generated/LaserPulse.LaserPulse_C|SetColor _returnvalue (Variables|Default|GetColor))
    (Variables|/Game/STAB/Blueprints/Generated/LaserPulse.LaserPulse_C|SetShooter _returnvalue self)))

(fn OverdriveToggle
  (params (Active :type Boolean))
  (bind _overdriveshine (Variables|Default|GetOverdriveShine))
  (bind _charactermovement (Variables|Character|GetCharacterMovement))
  (if Active
    (Audio|PlaySoundatLocation "/Game/STAB/Sounds/ForcefieldUp.ForcefieldUp" (Transformation|GetActorLocation) "0, 0, 0" 1.0 1.0 0.0 0 0 0)
    (Variables|/Script/Engine.CharacterMovementComponent|SetJumpZVelocity _charactermovement 1.2e+03)
    (Variables|/Script/Engine.CharacterMovementComponent|SetMaxWalkSpeed _charactermovement 1.5e+03)
    (Variables|Default|SetOverdrive true)
    (Rendering|Material|SetMaterial _overdriveshine 0 "/Game/STAB/Materials/Energy/GlowAura.GlowAura")
    (Rendering|Material|SetVectorParameterValueonMaterials _overdriveshine "Color" (Variables|Default|GetColor))
    (else
      (Variables|/Script/Engine.CharacterMovementComponent|SetJumpZVelocity _charactermovement 8e+02)
      (Variables|/Script/Engine.CharacterMovementComponent|SetMaxWalkSpeed _charactermovement 9e+02)
      (Variables|Default|SetOverdrive false)
      (Rendering|Material|SetMaterial _overdriveshine 0 "/Game/STAB/Materials/Invisible.Invisible"))))