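; AClassAgent is a player class that fires homing missiles and deploys an auto turret as its Overdrive ability.
; ToggleFire spawns a missile along the aim rotation and passes it shooter and color; ClassTick counts down the cooldown, and the missile Target assignment is disconnected.
; OverdriveToggle launches a colored turret forward with an impulse and keeps a reference to destroy it when Overdrive ends.
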(event EventBeginPlay)

(event Collision|EventActorBeginOverlap
  (params (OtherActor :type Actor%20Object%20Reference)))

(event EventTick
  (params (DeltaSeconds :type Float%20%28single-precision%29))
  (|CallParentFunction DeltaSeconds) ; This node is disabled and will not be called.\nDrag off pins to build functionality.
)

(fn ConstructionScript
  (|CallParentFunction))

(fn ToggleFire
  (params (Firing :type Boolean))
  (bind _firepoint (Variables|Default|GetFirePoint))
  (bind _returnvalue (Transformation|GetWorldLocation _firepoint))
  (if (and Firing (<= (Variables|Default|GetFiringCooldown) 0.0))
    (bind (_firerotator _firelocation) (CallFunction|GetFireRotator _returnvalue))
    (bind _returnvalue_2 (Game|SpawnActorfromClass "/Game/STAB/Blueprints/Generated/HomingMissile.HomingMissile_C" (Math|Transform|MakeTransform (+ (* (Math|Vector|GetForwardVector _firerotator) 2e+02) _returnvalue) _firerotator "1,1,1") "AdjustIfPossibleButDontSpawnIfColliding" 0 0))
    (if (Utilities|IsValid _returnvalue_2)
      (Variables|/Game/STAB/Blueprints/Generated/HomingMissile.HomingMissile_C|SetShooter _returnvalue_2 self)
      (Variables|/Game/STAB/Blueprints/Generated/HomingMissile.HomingMissile_C|SetColor _returnvalue_2 (Variables|Default|GetColor))
      (Variables|Default|SetFiringCooldown 0.5))))

(fn ClassTick
  (params (DeltaSeconds :type Float%20%28single-precision%29))
  (Variables|Default|SetFiringCooldown (- (Variables|Default|GetFiringCooldown) DeltaSeconds)))

(fn OverdriveToggle
  (params (Active :type Boolean))
  (bind _firepoint (Variables|Default|GetFirePoint))
  (bind _returnvalue (Math|Vector|GetForwardVector _firepoint))
  (if Active
    (bind _returnvalue_2 (Game|SpawnActorfromClass "/Game/STAB/Blueprints/Generated/AutoTurret.AutoTurret_C" (Math|Transform|MakeTransform (+ (Transformation|GetWorldLocation _firepoint) (* _returnvalue 1e+02)) (Math|Rotator|MakeRotator 0.0 0.0 (.yaw (Transformation|GetWorldRotation _firepoint))) "1,1,1") "AdjustIfPossibleButDontSpawnIfColliding" 0 0))
    (if (Utilities|IsValid _returnvalue_2)
      (Variables|/Game/STAB/Blueprints/Generated/AutoTurret.AutoTurret_C|SetColor _returnvalue_2 (Variables|Default|GetColor))
      (Physics|AddImpulse (Variables|/Game/STAB/Blueprints/Generated/AutoTurret.AutoTurret_C|GetAutoTurret _returnvalue_2) (* _returnvalue 1e+03) "None" true)
      (Variables|Default|SetOverdrive true)
      (Variables|Default|SetTurret _returnvalue_2))
    (else
      (Actor|DestroyActor (Variables|Default|GetTurret))
      (Variables|Default|SetOverdrive false))))