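; S-Class playable agent that fights with two launchable physics fists and can turn into a rolling hamster ball during Overdrive.
; ClassTick runs each fist's idle, launch and return states; fast fist or ball hits deal damage.
; Jump and fire within a short window trigger a fist jump, punching nearby floor for upward impulse.
; Overdrive swaps character movement for camera-relative ball physics with refreshed i-frames; timeslow boosts fist speed.
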(event Collision|EventHit
  (params (MyComp :type Primitive%20Component%20Object%20Reference) (Other :type Actor%20Object%20Reference) (OtherComp :type Primitive%20Component%20Object%20Reference) (bSelfMoved :type Boolean) (HitLocation :type Vector :default "0, 0, 0") (HitNormal :type Vector :default "0, 0, 0") (NormalImpulse :type Vector :default "0, 0, 0") (Hit :type Hit%20Result%20Structure%20%28by%20ref%29))
  (bind _fistlcapsule (Variables|Default|GetFistLCapsule))
  (bind _fistrcapsule (Variables|Default|GetFistRCapsule))
  (if (!= Other self)
    (if (>= (Utilities|Array|FindItem (Utilities|Array|MakeArray (Variables|Default|GetFistRCapsule) (Variables|Default|GetFistLCapsule) (Variables|Default|GetHamsterBall)) MyComp) 0)
      (if (> (Math|Vector|VectorLength (Transformation|GetComponentVelocity MyComp)) 3e+02)
        (Game|Damage|ApplyPointDamage Other 2.0 HitLocation Hit 0 self "/Script/Engine.DamageType"))
      (if (== MyComp _fistrcapsule)
        (switch int (Variables|Default|GetFistRState)
          (:1
            (Variables|Default|SetRStruck true)
            (Utilities|FlowControl|Delay 0.5)
            (if (and (== (Variables|Default|GetFistRState) 1) (Variables|Default|GetRStruck))
              (Variables|Default|SetFistRState 2)
              (Variables|Default|SetRStruck false)))
          (:2
            (Collision|SetCollisionEnabled _fistrcapsule "QueryOnly")))
        (elif (== MyComp _fistlcapsule)
          (switch int (Variables|Default|GetFistLState)
            (:1
              (Variables|Default|SetLStruck true)
              (Utilities|FlowControl|Delay 0.5)
              (if (and (== (Variables|Default|GetFistLState) 1) (Variables|Default|GetLStruck))
                (Variables|Default|SetFistLState 2)
                (Variables|Default|SetLStruck false)))
            (:2
              (Collision|SetCollisionEnabled _fistlcapsule "QueryOnly"))))))))

(event Input|ActionEvents|InputActionJump
  (params (Key :type Key%20Structure))
  (bind _hamsterball (Variables|Default|GetHamsterBall))
  (bind _returnvalue (Transformation|GetWorldLocation _hamsterball))
  (:Pressed
    (bind _jump (CallFunction|TryFistJump))
    (if _jump
      (Variables|Default|SetFistJumpWindow 0.1))
    (Character|Jump)
    (if (Variables|Default|GetOverdrive)
      (bind (_outhit _returnvalue_2) (Collision|SphereTraceForObjects _returnvalue (+ _returnvalue "0, 0,-50.000000") 9e+01 (Utilities|Array|MakeArray "ObjectTypeQuery1" "ObjectTypeQuery2" "ObjectTypeQuery5" "ObjectTypeQuery6") false 0 "None"))
      (if _returnvalue_2
        (Physics|AddImpulse _hamsterball (* (.impactnormal _outhit) 1e+03) "None" true))))
  (:Released
    (Character|StopJumping)))

(fn ConstructionScript
  (|CallParentFunction)
  (Rendering|Material|SetVectorParameterValueonMaterials (Variables|Default|GetFistRMesh) "Color" (Variables|Default|GetColor)))

(fn ClassTick
  (params (DeltaSeconds :type Float%20%28single-precision%29))
  (bind _fistrcapsule (Variables|Default|GetFistRCapsule))
  (bind _fistlpoint (Variables|Default|GetFistLPoint))
  (bind _fistltarget (Variables|Default|GetFistLTarget))
  (bind _fistrpoint (Variables|Default|GetFistRPoint))
  (bind _fistrtarget (Variables|Default|GetFistRTarget))
  (bind _fistlcapsule (Variables|Default|GetFistLCapsule))
  (bind _hamsterball (Variables|Default|GetHamsterBall))
  (bind _returnvalue (Transformation|GetWorldLocation _fistrpoint))
  (bind _returnvalue_2 (Transformation|GetWorldLocation _fistrcapsule))
  (bind _returnvalue_3 (Transformation|GetWorldLocation _fistlpoint))
  (bind _returnvalue_4 (Transformation|GetWorldLocation _fistlcapsule))
  (Utilities|FlowControl|Sequence
    (:then_0
      (switch int (Variables|Default|GetFistLState)
        (:0
          (Transformation|SetWorldLocation _fistlcapsule _returnvalue_3 false false)
          (Physics|SetPhysicsLinearVelocity _fistlcapsule "0, 0, 0" false "None")
          (Transformation|SetWorldRotation _fistlcapsule (Math|Interpolation|RInterpTo (Transformation|GetWorldRotation _fistlcapsule) (Transformation|GetWorldRotation (Variables|Default|GetFistAim)) DeltaSeconds 1e+01) false false))
        (:1
          (Physics|SetPhysicsLinearVelocity _fistlcapsule (* (Math|Vector|GetForwardVector (Math|Rotator|FindLookatRotation _returnvalue_4 _fistltarget)) (Variables|Default|GetFistSpeed)) true "None")
          (if (<= (Math|Vector|Distance(Vector) _returnvalue_4 _fistltarget) (Variables|Default|GetFistSnap))
            (Variables|Default|SetFistLState 2)
            (Variables|Default|SetLStruck false)))
        (:2
          (Physics|SetPhysicsLinearVelocity _fistlcapsule (* (Math|Vector|GetForwardVector (Math|Rotator|FindLookatRotation _returnvalue_4 _returnvalue_3)) (* (Variables|Default|GetFistSpeed) 6.0)) false "None")
          (if (<= (Math|Vector|Distance(Vector) _returnvalue_4 _returnvalue_3) (Variables|Default|GetFistSnap))
            (Variables|Default|SetFistLState 0)
            (Collision|SetCollisionEnabled _fistlcapsule "QueryAndPhysics")
            (Variables|Default|SetLStruck false)))))
    (:then_1
      (switch int (Variables|Default|GetFistRState)
        (:0
          (Transformation|SetWorldLocation _fistrcapsule _returnvalue false false)
          (Physics|SetPhysicsLinearVelocity _fistrcapsule "0, 0, 0" false "None")
          (Transformation|SetWorldRotation _fistrcapsule (Math|Interpolation|RInterpTo (Transformation|GetWorldRotation _fistrcapsule) (Transformation|GetWorldRotation (Variables|Default|GetFistAim)) DeltaSeconds 1e+01) false false))
        (:1
          (Physics|SetPhysicsLinearVelocity _fistrcapsule (* (Math|Vector|GetForwardVector (Math|Rotator|FindLookatRotation _returnvalue_2 _fistrtarget)) (Variables|Default|GetFistSpeed)) true "None")
          (if (<= (Math|Vector|Distance(Vector) _returnvalue_2 _fistrtarget) (Variables|Default|GetFistSnap))
            (Variables|Default|SetFistRState 2)
            (Variables|Default|SetRStruck false)))
        (:2
          (Physics|SetPhysicsLinearVelocity _fistrcapsule (* (Math|Vector|GetForwardVector (Math|Rotator|FindLookatRotation _returnvalue_2 _returnvalue)) (* (Variables|Default|GetFistSpeed) 6.0)) false "None")
          (if (<= (Math|Vector|Distance(Vector) _returnvalue_2 _returnvalue) (Variables|Default|GetFistSnap))
            (Variables|Default|SetFistRState 0)
            (Collision|SetCollisionEnabled _fistrcapsule "QueryAndPhysics")
            (Variables|Default|SetRStruck false)))))
    (:then_2
      (if (Variables|Default|GetOverdrive)
        (Transformation|SetActorLocationAndRotation (Transformation|GetWorldLocation _hamsterball) (Transformation|GetWorldRotation _hamsterball))
        (bind _onground (CallFunction|RollingonGround))
        (Physics|AddForce (Variables|Default|GetHamsterBall) (* (Math|Vector|RotateVectorAroundAxis (Math|Vector|MakeVector (Input|AxisValues|GetMoveForward) (Input|AxisValues|GetMoveRight) 0.0) (.yaw (Transformation|GetWorldRotation (Variables|Default|GetFollowCamera))) "0, 0,1.000000") (+ (* (Math|Conversions|ToFloat(Boolean) _onground) 5e+02) 3e+02)) "None" true)
        (Variables|Default|SetiFrames 0.1)
        (else
          (Transformation|SetWorldLocationAndRotation _hamsterball (Transformation|GetActorLocation) (Transformation|GetActorRotation) false false))))
    (:then_3
      (Variables|Default|SetFistJumpWindow (- (Variables|Default|GetFistJumpWindow) DeltaSeconds)))))

(fn ToggleFire
  (params (Firing :type Boolean))
  (bind _fistsnap (Variables|Default|GetFistSnap))
  (bind _returnvalue (* _fistsnap 0.2))
  (if Firing
    (if (and (== (Variables|Default|GetFistLState) 0) (== (Variables|Default|GetFistRState) 0))
      (bind _jump (CallFunction|TryFistJump))
      (if (not _jump)
        (Variables|Default|SetFistJumpWindow 0.1)
        (if (== (Variables|Default|GetFistRState) 0) :!label _label
          (bind (_firerotator _firelocation) (CallFunction|GetFireRotator (Transformation|GetWorldLocation (Variables|Default|GetFistRPoint))))
          (Variables|Default|SetFistRTarget (+ _firelocation (* (Math|Vector|GetForwardVector _firerotator) _returnvalue)))
          (Variables|Default|SetFistRState 1)
          (elif (== (Variables|Default|GetFistLState) 0)
            (bind (_firerotator_2 _firelocation_2) (CallFunction|GetFireRotator (Transformation|GetWorldLocation (Variables|Default|GetFistLPoint))))
            (Variables|Default|SetFistLTarget (+ _firelocation_2 (* (Math|Vector|GetForwardVector _firerotator_2) _returnvalue)))
            (Variables|Default|SetFistLState 1))))
      (else
        (goto _label)))))

(fn OverdriveToggle
  (params (Active :type Boolean))
  (bind _charactermovement (Variables|Character|GetCharacterMovement))
  (bind _perceivedvelocity (Variables|Default|GetPerceivedVelocity))
  (bind _hamsterball (Variables|Default|GetHamsterBall))
  (bind _capsulecomponent (Variables|Default|GetCapsuleComponent))
  (if Active
    (Variables|Default|SetOverdrive true)
    (Components|Activation|Deactivate _charactermovement)
    (Physics|SetSimulatePhysics _hamsterball true)
    (Rendering|SetVisibility _hamsterball true false)
    (Collision|SetCollisionEnabled _hamsterball "QueryAndPhysics")
    (Collision|SetCollisionResponsetoChannel _capsulecomponent "ECC_Vehicle" "ECR_Overlap")
    (Physics|SetPhysicsLinearVelocity (Variables|Default|GetHamsterBall) _perceivedvelocity false "None")
    (else
      (Variables|Default|SetOverdrive false)
      (Components|Activation|Activate _charactermovement false)
      (Physics|SetSimulatePhysics _hamsterball false)
      (Rendering|SetVisibility _hamsterball false false)
      (Collision|SetCollisionEnabled _hamsterball "NoCollision")
      (Collision|SetCollisionResponsetoChannel _capsulecomponent "ECC_Vehicle" "ECR_Block")
      (Transformation|SetActorRotation (Math|Rotator|MakeRotator 0.0 0.0 (.yaw (Transformation|GetActorRotation))))
      (Variables|/Script/Engine.MovementComponent|SetVelocity (Variables|Character|GetCharacterMovement) _perceivedvelocity))))

(fn TimeslowActivate
  (params (Slow :type Boolean))
  (|CallParentFunction Slow)
  (if Slow
    (Variables|Default|SetFistSpeed 1e+04)
    (else
      (Variables|Default|SetFistSpeed 1e+03))))

(fn RollingonGround
  (bind _returnvalue (Collision|SphereOverlapActors (+ (Transformation|GetWorldLocation (Variables|Default|GetHamsterBall)) "0, 0,-50.000000") 9e+01 (Utilities|Array|MakeArray "ObjectTypeQuery1" "ObjectTypeQuery2" "ObjectTypeQuery5" "ObjectTypeQuery6") 0 (Utilities|Array|MakeArray self)))
  (return _returnvalue))

(fn TryFistJump
  (bind _returnvalue (Math|Vector|VectorDown))
  (bind _returnvalue_2 (Math|Vector|VectorDown))
  (bind _array (Utilities|Array|MakeArray "ObjectTypeQuery1" "ObjectTypeQuery2" "ObjectTypeQuery3" "ObjectTypeQuery5" "ObjectTypeQuery6"))
  (bind _punchfloordistance (Variables|Default|GetPunchFloorDistance))
  (bind _fistlpoint (Variables|Default|GetFistLPoint))
  (bind _fistrpoint (Variables|Default|GetFistRPoint))
  (bind _punchfloordistance_2 (Variables|Default|GetPunchFloorDistance))
  (bind _returnvalue_3 (* _returnvalue _punchfloordistance))
  (bind _returnvalue_4 (Transformation|GetWorldLocation _fistrpoint))
  (bind _returnvalue_5 (Transformation|GetWorldLocation _fistlpoint))
  (bind _returnvalue_6 (* _punchfloordistance_2 1.2))
  (bind _returnvalue_7 (* _returnvalue_2 _returnvalue_6))
  (if (> (Variables|Default|GetFistJumpWindow) 0.0)
    (bind _returnvalue_8 (Collision|LineTraceForObjects _returnvalue_5 (+ _returnvalue_5 _returnvalue_3) _array false 0 "None"))
    (if _returnvalue_8
      (bind _returnvalue_9 (Collision|LineTraceForObjects _returnvalue_4 (+ _returnvalue_4 _returnvalue_3) _array false 0 "None"))
      (if _returnvalue_9
        (LocalVariables|SetPunchVector _returnvalue_2)
        (Variables|Default|SetFistLTarget (+ (Transformation|GetWorldLocation (Variables|Default|GetFistLPoint)) _returnvalue_7))
        (Variables|Default|SetFistRTarget (+ (Transformation|GetWorldLocation (Variables|Default|GetFistRPoint)) _returnvalue_7))
        (Variables|Default|SetFistLState 1)
        (Variables|Default|SetFistRState 1)
        (Physics|AddImpulse (Variables|Character|GetCharacterMovement) (* (LocalVariables|GetPunchVector) -1.5e+03) true)
        (Physics|AddImpulse (Variables|Default|GetHamsterBall) (* (LocalVariables|GetPunchVector) -1.5e+03) "None" true)
        (return true)
        (else
          _)))
    (return false)
    (else
      (return false))))