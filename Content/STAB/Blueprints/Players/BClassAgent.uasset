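; Agent player class that lobs chemical bombs and gains wings during Overdrive.
; Firing spawns a color-tagged bomb and launches it along the aim rotation, with upward lift scaled by target distance, then starts a short cooldown.
; ClassTick counts down that cooldown and, in Overdrive, eases vertical velocity toward a glide limit.
; Holding jump adds capped upward thrust that drains the Overdrive meter; toggling Overdrive shows or hides the colored wing marker.
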(event Input|ActionEvents|InputActionJump
  (params (Key :type Key%20Structure))
  (:Pressed
    (Character|Jump)
    (Variables|Default|SetJumpHeld true))
  (:Released
    (Character|StopJumping)
    (Variables|Default|SetJumpHeld false)))

(fn ConstructionScript
  (|CallParentFunction))

(fn ToggleFire
  (params (Firing :type Boolean))
  (bind _firepoint (Variables|Default|GetFirePoint))
  (bind _returnvalue (Transformation|GetWorldLocation _firepoint))
  (if Firing
    (if (<= (Variables|Default|GetFireCooldown) 0.0)
      (bind (_firerotator _firelocation) (CallFunction|GetFireRotator _returnvalue))
      (LocalVariables|SetFireRotator _firerotator)
      (LocalVariables|SetFireVector (+ (* (Math|Vector|GetForwardVector _firerotator) 6e+03) (Math|Vector|MakeVector 0.0 0.0 (* (Math|Vector|Distance(Vector) _firelocation _returnvalue) 0.08))))
      (bind _returnvalue_2 (Game|SpawnActorfromClass "/Game/STAB/Blueprints/Generated/ChemicalBomb.ChemicalBomb_C" (Math|Transform|MakeTransform (+ (* (Math|Vector|GetForwardVector (LocalVariables|GetFireRotator)) 1e+02) (Transformation|GetWorldLocation (Variables|Default|GetFirePoint))) "0, 0, 0" "0.300000,0.300000,0.300000") "AdjustIfPossibleButDontSpawnIfColliding" 0 0))
      (if (Utilities|IsValid _returnvalue_2)
        (Physics|AddImpulse (Variables|/Game/STAB/Blueprints/Generated/ChemicalBomb.ChemicalBomb_C|GetSphere _returnvalue_2) (LocalVariables|GetFireVector) "None" true)
        (Variables|/Game/STAB/Blueprints/Generated/ChemicalBomb.ChemicalBomb_C|SetColor _returnvalue_2 (Variables|Default|GetColor))
        (Variables|/Game/STAB/Blueprints/Generated/ChemicalBomb.ChemicalBomb_C|SetShooter _returnvalue_2 self)
        (Variables|Default|SetFireCooldown 0.5)))))

(fn ClassTick
  (params (DeltaSeconds :type Float%20%28single-precision%29))
  (bind _charactermovement (Variables|Character|GetCharacterMovement))
  (bind _maxwingfall (LocalVariables|GetMaxWingFall))
  (Variables|Default|SetFireCooldown (- (Variables|Default|GetFireCooldown) DeltaSeconds))
  (if (Variables|Default|GetOverdrive)
    (if (<= (.z (Variables|/Script/Engine.MovementComponent|GetVelocity _charactermovement)) _maxwingfall)
      (Variables|/Script/Engine.MovementComponent|SetVelocity _charactermovement (Math|Vector|MakeVector (.x (Variables|/Script/Engine.MovementComponent|GetVelocity _charactermovement)) (.y (Variables|/Script/Engine.MovementComponent|GetVelocity _charactermovement)) (Math|Interpolation|FInterpTo (.z (Variables|/Script/Engine.MovementComponent|GetVelocity _charactermovement)) _maxwingfall DeltaSeconds 5.0))))
    (if (Variables|Default|GetJumpHeld)
      (if (<= (.z (Variables|/Script/Engine.MovementComponent|GetVelocity _charactermovement)) (* _maxwingfall -3.0))
        (Physics|AddForce (Variables|Character|GetCharacterMovement) "0, 0,300000.000000")
        (Variables|Default|SetOverdriveMeter (- (Variables|Default|GetOverdriveMeter) (/ DeltaSeconds 7.0)))))))

(fn OverdriveToggle
  (params (Active :type Boolean))
  (bind _wingmarker (Variables|Default|GetWingMarker))
  (bind _output_get (Variables|Default|SetOverdrive Active))
  (if _output_get
    (Rendering|Material|SetMaterial _wingmarker 0 "/Game/STAB/Materials/Energy/Transparent.Transparent")
    (Rendering|Material|SetVectorParameterValueonMaterials _wingmarker "Color" (Variables|Default|GetColor))
    (else
      (Rendering|Material|SetMaterial _wingmarker 0 "/Game/STAB/Materials/Invisible.Invisible"))))