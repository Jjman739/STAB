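; Suzerain is a playable character class that fires colored laser pulses and uses a short forward teleport as its Overdrive.
; ClassTick runs a cooldown while fire is held, spawning randomly colored LaserPulse actors from FirePoint along the aim rotation.
; OverdriveToggle makes a swept jump along FirePoint's forward vector with a slight lift.
; A successful jump drains some meter, clears Overdrive and plays teleport effects at both ends.
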(event EventBeginPlay)

(event Collision|EventActorBeginOverlap
  (params (OtherActor :type Actor%20Object%20Reference)))

(event EventTick
  (params (DeltaSeconds :type Float%20%28single-precision%29))
  (|CallParentFunction DeltaSeconds) ; This node is disabled and will not be called.\nDrag off pins to build functionality.
)

(fn ConstructionScript
  (|CallParentFunction))

(fn ToggleFire
  (params (Firing :type Boolean)))

(fn ClassTick
  (params (DeltaSeconds :type Float%20%28single-precision%29))
  (bind _output_get (Variables|Default|SetLaserCooldown (- (Variables|Default|GetLaserCooldown) DeltaSeconds)))
  (if (and (Variables|Default|GetShootHeld) (<= _output_get 0.0))
    (bind _firerotator (CallFunction|GetFireRotator (Transformation|GetWorldLocation (Variables|Default|GetFirePoint))))
    (Variables|Default|SetLaserCooldown 0.25)
    (bind _returnvalue (Game|SpawnActorfromClass "/Game/STAB/Blueprints/Generated/LaserPulse.LaserPulse_C" (Math|Transform|MakeTransform (+ (* (Math|Vector|GetForwardVector _firerotator) 5e+01) (Transformation|GetWorldLocation (Variables|Default|GetFirePoint))) _firerotator "1,1,1") "AlwaysSpawn" 0 0))
    (Variables|/Game/STAB/Blueprints/Generated/LaserPulse.LaserPulse_C|SetColor _returnvalue (.OutItem (Utilities|Array|Random (Variables|Default|GetColorChoices))))
    (Variables|/Game/STAB/Blueprints/Generated/LaserPulse.LaserPulse_C|SetShooter _returnvalue self)))

(fn OverdriveToggle
  (params (Active :type Boolean))
  (bind _returnvalue (Transformation|GetActorLocation))
  (LocalVariables|SetOriginalLocation _returnvalue)
  (bind _returnvalue_2 (Transformation|SetActorLocation (+ (+ _returnvalue (* (Math|Vector|GetForwardVector (Variables|Default|GetFirePoint)) 1.5e+03)) "0,0.000000,50.000000") true true))
  (if _returnvalue_2
    (Variables|Default|SetOverdriveMeter (- (Variables|Default|GetOverdriveMeter) 0.07))
    (Variables|Default|SetOverdrive false)
    (Effects|SpawnEmitteratLocation "/Game/STAB/Particles/SuzerainTeleport.SuzerainTeleport" (Transformation|GetActorLocation))
    (Effects|SpawnEmitteratLocation "/Game/STAB/Particles/SuzerainTeleport.SuzerainTeleport" (LocalVariables|GetOriginalLocation))))