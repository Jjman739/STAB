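; Base pickup actor that rotates, hovers and is consumed when a StabTemplate actor overlaps it.
; Each tick a downward sphere trace switches the vertical force on the physics sphere between up and down to keep it floating above surfaces.
; Overlap calls the empty PickedUp hook, plays a sound and destroys the pickup.
; Permanent pickups call the empty PermaSpawn hook, others expire after a fixed lifespan; construction tints the sphere.
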(event EventBeginPlay
  (if (Variables|Default|GetPermanent)
    (CallFunction|PermaSpawn)
    (else
      (Actor|SetLifeSpan 3e+01))))

(event EventTick
  (params (DeltaSeconds :type Float%20%28single-precision%29))
  (bind _returnvalue (Transformation|GetActorLocation))
  (bind _sphere (Variables|Default|GetSphere))
  (Class|Actor|AddActorWorldRotation (Math|Rotator|MakeRotator 0.0 0.0 (* DeltaSeconds 1e+02)))
  (bind _returnvalue_2 (Collision|SphereTraceForObjects _returnvalue (+ _returnvalue "0, 0,-50.000000") 25.0 (Utilities|Array|MakeArray "ObjectTypeQuery1" "ObjectTypeQuery2") false 0 "None"))
  (if _returnvalue_2
    (Physics|AddForce _sphere "0, 0,300.000000" "None" true)
    (else
      (Physics|AddForce _sphere "0, 0,-300.000000" "None" true))))

(event Collision|EventActorBeginOverlap
  (params (OtherActor :type Actor%20Object%20Reference))
  (bind _asstab_template (Utilities|Casting|CastToStabTemplate OtherActor))
  (CallFunction|PickedUp _asstab_template)
  (Audio|PlaySoundatLocation "/Game/STAB/Sounds/ForcefieldUp.ForcefieldUp" (Transformation|GetActorLocation) "0, 0, 0" 1.0 1.0 0.0 0 0 0)
  (Actor|DestroyActor))

(fn ConstructionScript
  (Rendering|Material|SetVectorParameterValueonMaterials (Variables|Default|GetSphere) "Color" (Variables|Default|GetSphereColor)))

(fn PickedUp
  (params (Player :type Stab%20Template%20Object%20Reference)))

(fn PermaSpawn)