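; Abstract weak point for bosses that passes the damage it takes on to the Boss it is parented to.
; BeginPlay initializes HP and links the parent Boss.
; Each hit subtracts damage, capped at remaining HP and scaled by DamageMult, from the boss.
; Unless MaxHP is -1, it also tracks its own HP, awards hurt or kill credit, and on depletion deals bonus boss damage and destroys itself, spawning a death particle.
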(event Game|Damage|EventAnyDamage
  (params (Damage :type Float%20%28single-precision%29) (DamageType :type Damage%20Type%20Object%20Reference) (InstigatedBy :type Controller%20Object%20Reference) (DamageCauser :type Actor%20Object%20Reference))
  (bind _returnvalue (Transformation|GetActorLocation))
  (bind _linkedboss (Variables|Default|GetLinkedBoss))
  (bind _linkedboss_2 (Variables|Default|GetLinkedBoss))
  (Variables|/Game/STAB/Blueprints/Abstract/Boss.Boss_C|SetHP _linkedboss (- (Variables|/Game/STAB/Blueprints/Abstract/Boss.Boss_C|GetHP _linkedboss) (* (Math|Float|Clamp(Float) Damage 0.0 (Variables|Default|GetHP)) (Variables|Default|GetDamageMult))))
  (if (!= (Variables|Default|GetMaxHP) -1.0)
    (bind _output_get (Variables|Default|SetHP (- (Variables|Default|GetHP) Damage)))
    (if (<= _output_get 0.0)
      (CallFunction|GiveKillCredit DamageCauser _returnvalue)
      (Variables|/Game/STAB/Blueprints/Abstract/Boss.Boss_C|SetHP _linkedboss_2 (- (Variables|/Game/STAB/Blueprints/Abstract/Boss.Boss_C|GetHP _linkedboss_2) (Variables|Default|GetDestructionDamage)))
      (Actor|DestroyActor)
      (else
        (CallFunction|GiveHurtCredit DamageCauser _returnvalue)))))

(event EventBeginPlay
  (bind _returnvalue (Actor|GetParentActor))
  (bind _maxhp (Variables|Default|GetMaxHP))
  (if (!= _maxhp -1.0)
    (Variables|Default|SetHP _maxhp))
  (if (Utilities|IsValid _returnvalue)
    (bind _asboss (Utilities|Casting|CastToBoss _returnvalue))
    (Variables|Default|SetLinkedBoss _asboss)))

(event EventDestroyed
  (Effects|SpawnEmitteratLocation (Variables|Default|GetDeathParticle) (Transformation|GetActorLocation)))

(fn ConstructionScript)