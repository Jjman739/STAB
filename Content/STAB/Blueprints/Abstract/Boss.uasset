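; Abstract boss base Blueprint that tracks health and gives each boss an on-screen HUD.
; On BeginPlay it creates a BossHUD widget bound to itself, adds it to the player screen and sets HP to MaxHP.
; AnyDamage subtracts the square of the incoming damage from HP, with no death handling or clamping in this graph.
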(event EventBeginPlay
  (bind _returnvalue (UserInterface|CreateWidget "/Game/STAB/UI/BossHUD.BossHUD_C"))
  (Variables|/Game/STAB/UI/BossHUD.BossHUD_C|SetBoss _returnvalue self)
  (UserInterface|Viewport|AddtoPlayerScreen _returnvalue)
  (Variables|Default|SetHP (Variables|Default|GetMaxHP)))

(event Game|Damage|EventAnyDamage
  (params (Damage :type Float%20%28single-precision%29) (DamageType :type Damage%20Type%20Object%20Reference) (InstigatedBy :type Controller%20Object%20Reference) (DamageCauser :type Actor%20Object%20Reference))
  (Variables|Default|SetHP (- (Variables|Default|GetHP) (* Damage (Variables|Default|GetDamage%25)))))

(fn ConstructionScript
  (|CallParentFunction))