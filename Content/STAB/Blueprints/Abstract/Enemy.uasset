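; Abstract base enemy that rewards its attacker on hurt and death through credit functions.
; GiveHurtCredit raises a StabTemplate attacker's Overdrive meter.
; GiveKillCredit reuses that, rolls a pickup drop for a StabTemplate killer, and reports the enemy's class to the first Scorekeeper found.
; DropPickup uses weighted chance, favoring life when the player's HP is low, otherwise possibly energy when Overdrive is not near full.
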(event Game|Damage|EventAnyDamage
  (params (Damage :type Float%20%28single-precision%29) (DamageType :type Damage%20Type%20Object%20Reference) (InstigatedBy :type Controller%20Object%20Reference) (DamageCauser :type Actor%20Object%20Reference)))

(fn ConstructionScript)

(fn GiveHurtCredit
  (params (Attacker :type Actor%20Object%20Reference) (HurtPoint :type Vector))
  (bind _asstab_template (Utilities|Casting|CastToStabTemplate Attacker))
  (Variables|/Game/STAB/Blueprints/Abstract/StabTemplate.StabTemplate_C|SetOverdriveMeter _asstab_template (+ (Variables|/Game/STAB/Blueprints/Abstract/StabTemplate.StabTemplate_C|GetOverdriveMeter _asstab_template) 0.07)))

(fn GiveKillCredit
  (params (Killer :type Actor%20Object%20Reference) (HurtPoint :type Vector))
  (CallFunction|GiveHurtCredit Killer HurtPoint)
  (Utilities|FlowControl|Sequence
    (:then_0
      (bind _asstab_template (Utilities|Casting|CastToStabTemplate Killer))
      (CallFunction|DropPickup _asstab_template))
    (:then_1
      (bind _outactors (Actor|GetAllActorsOfClass "/Game/STAB/Blueprints/Utility/Scorekeeper.Scorekeeper_C"))
      (if (Utilities|Array|IsValidIndex _outactors)
        (Default|GiveEnemyCredit (Utilities|Array|Get(acopy) _outactors) (Utilities|GetClass self))))))

(fn DropPickup
  (params (Player :type Stab%20Template%20Object%20Reference))
  (LocalVariables|SetPickupTransform (Math|Transform|MakeTransform (Transformation|GetActorLocation) "0, 0, 0" "0.500000,0.500000,0.500000"))
  (if (< (Variables|/Game/STAB/Blueprints/Abstract/StabTemplate.StabTemplate_C|GetHP Player) 5)
    (if (Math|Random|RandomBoolwithWeight 0.3)
      (Game|SpawnActorfromClass "/Game/STAB/Blueprints/Utility/LifePickup.LifePickup_C" (LocalVariables|GetPickupTransform) "AdjustIfPossibleButDontSpawnIfColliding" 0 0)
      (return true)
      (else
        _)))
  (if (< (Variables|/Game/STAB/Blueprints/Abstract/StabTemplate.StabTemplate_C|GetOverdriveMeter Player) 0.8)
    (if (Math|Random|RandomBoolwithWeight 0.2)
      (Game|SpawnActorfromClass "/Game/STAB/Blueprints/Utility/EnergyPickup.EnergyPickup_C" (LocalVariables|GetPickupTransform) "AdjustIfPossibleButDontSpawnIfColliding" 0 0)
      (return true)
      (else
        _)))
  (return false))