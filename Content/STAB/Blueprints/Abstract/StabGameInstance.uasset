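; Game instance for S.T.A.B. that sets the window title on init and launches stages with a chosen character.
; LaunchStage resolves character and level from name-keyed lookup maps, records both selections, then opens the level by object reference.
; It also resets the ability count map for Forcefield, Timeslow and Hack on each launch.
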(event EventInit
  (Class|KismetSystemLibrary|SetWindowTitle (Utilities|Text|MakeLiteralText "S.T.A.B.: The Video Game")))

(fn LaunchStage
  (params (StageName :type String) (CharacterName :type String))
  (Variables|Default|SetSelectedCharacter (.Value (Utilities|Map|Find (Variables|Default|GetCharacterList) CharacterName)))
  (Variables|Default|SetLastLevelName StageName)
  (Variables|Default|SetLastCharacterName CharacterName)
  (Game|OpenLevel(byObjectReference) (.Value (Utilities|Map|Find (Variables|Default|GetLevelList) StageName)))
  (Variables|Default|SetAbilityCounts (Utilities|Map|MakeMap "Forcefield" 5 "Timeslow" 5 "Hack" 5)))