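; Bounce pad actor that launches whatever overlaps it along its own up vector, scaled by an Impulse value.
; Characters receive a velocity-change impulse through their movement component, and SClassAgent characters also get one on their HamsterBall.
; Other actors receive the same impulse on their root primitive component, so rotating the pad changes the launch direction.
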(event Collision|EventActorBeginOverlap
  (params (OtherActor :type Actor%20Object%20Reference))
  (bind _returnvalue (Transformation|GetActorUpVector))
  (bind _impulse (Variables|Default|GetImpulse))
  (bind _returnvalue_2 (* _returnvalue _impulse))
  (bind _ascharacter (Utilities|Casting|CastToCharacter OtherActor)
    (:then
      (Physics|AddImpulse (Variables|/Script/Engine.Character|GetCharacterMovement _ascharacter) _returnvalue_2 true)
      (bind _assclass_agent (Utilities|Casting|CastToSClassAgent OtherActor))
      (Physics|AddImpulse (Variables|/Game/STAB/Blueprints/Players/SClassAgent.SClassAgent_C|GetHamsterBall _assclass_agent) _returnvalue_2 "None" true))
    (:CastFailed
      (bind _asprimitive_component (Utilities|Casting|CastToPrimitiveComponent (Variables|/Script/Engine.Actor|GetRootComponent OtherActor)))
      (Physics|AddImpulse _asprimitive_component _returnvalue_2 "None" true))))

(fn ConstructionScript)