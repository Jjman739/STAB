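; A sliding door actor that moves its Block component between an open point and a closed point.
; Every Tick interpolates the block's world location at constant Speed toward OpenPoint when Active is true, otherwise toward ClosedPoint.
; The target is picked without a branch by weighting both point locations with the Active bool converted to float.
; The move does not sweep for collision, and this file never changes Active itself.
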(event EventTick
  (params (DeltaSeconds :type Float%20%28single-precision%29))
  (bind _block (Variables|Default|GetBlock))
  (bind _active (Variables|Default|GetActive))
  (Transformation|SetWorldLocation _block (Math|Interpolation|VInterptoConstant (Transformation|GetWorldLocation _block) (+ (* (Transformation|GetWorldLocation (Variables|Default|GetClosedPoint)) (Math|Conversions|ToFloat(Boolean) (not _active))) (* (Transformation|GetWorldLocation (Variables|Default|GetOpenPoint)) (Math|Conversions|ToFloat(Boolean) _active))) DeltaSeconds (Variables|Default|GetSpeed)) false false))

(fn ConstructionScript)