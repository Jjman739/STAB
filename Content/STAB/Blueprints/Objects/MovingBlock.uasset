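; MovingBlock is an object whose block travels in a continuous loop through a set of waypoints while it is active.
; BeginPlay targets Point1, then Tick moves the Block toward the current point at constant Speed using VInterpToConstant, without sweeping.
; On coming close to the target, it selects the next child component of MovementPoints, wrapping to the first after the last.
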(event EventBeginPlay
  (Variables|Default|SetNextPoint (Variables|Default|GetPoint1)))

(event EventTick
  (params (DeltaSeconds :type Float%20%28single-precision%29))
  (bind _block (Variables|Default|GetBlock))
  (bind _movementpoints (Variables|Default|GetMovementPoints))
  (bind _children (Components|GetChildrenComponents _movementpoints true))
  (bind _returnvalue (Transformation|GetWorldLocation _block))
  (if (Variables|Default|GetActive)
    (Transformation|SetWorldLocation _block (Math|Interpolation|VInterptoConstant _returnvalue (Transformation|GetWorldLocation (Variables|Default|GetNextPoint)) DeltaSeconds (Variables|Default|GetSpeed)) false false)
    (if (<= (Math|Vector|Distance(Vector) _returnvalue (Transformation|GetWorldLocation (Variables|Default|GetNextPoint))) 1e+01)
      (if (== (Utilities|Array|Length _children) (+ (Utilities|Array|FindItem _children (Variables|Default|GetNextPoint)) 1))
        (Variables|Default|SetNextPoint (Utilities|Array|Get(acopy) _children))
        (else
          (Variables|Default|SetNextPoint (Utilities|Array|Get(acopy) _children (+ (Utilities|Array|FindItem _children (Variables|Default|GetNextPoint)) 1))))))))

(fn ConstructionScript)