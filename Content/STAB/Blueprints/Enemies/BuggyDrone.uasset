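; BuggyDrone is an enemy that chases the player on a physics-driven Buggy component, snapping the actor to its location every tick.
; With the player in range and visible, it predicts a lead point from velocity and distance.
; It fires colored laser bolts when that point is near, otherwise steers and pushes the buggy toward it.
; Any damage destroys it with kill credit, and its pickup logic can fall back to a random HackableDrone drop.
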(event Game|Damage|EventAnyDamage
  (params (Damage :type Float%20%28single-precision%29) (DamageType :type Damage%20Type%20Object%20Reference) (InstigatedBy :type Controller%20Object%20Reference) (DamageCauser :type Actor%20Object%20Reference))
  (bind _returnvalue (Transformation|GetActorLocation))
  (Effects|SpawnEmitteratLocation "/Game/STAB/Particles/Explosion.Explosion" _returnvalue)
  (CallFunction|GiveKillCredit DamageCauser _returnvalue)
  (Actor|DestroyActor))

(event EventTick
  (params (DeltaSeconds :type Float%20%28single-precision%29))
  (bind _returnvalue (Game|Player|GetPlayerPawn 0))
  (bind _returnvalue_2 (Transformation|GetActorRotation))
  (bind _returnvalue_3 (Game|Player|GetPlayerPawn 0))
  (bind _buggy (Variables|Default|GetBuggy))
  (bind _returnvalue_4 (Transformation|GetActorLocation _returnvalue_3))
  (bind _returnvalue_5 (Transformation|GetDistanceTo _returnvalue_3))
  (bind _returnvalue_6 (* _returnvalue_5 0.0004))
  (Transformation|SetActorLocation (Transformation|GetWorldLocation (Variables|Default|GetBuggy)) false false)
  (Utilities|FlowControl|Sequence
    (:then_0
      (if (<= (Transformation|GetDistanceTo _returnvalue) (Variables|Default|GetDetectionRange))
        (bind _returnvalue_7 (Collision|LineTraceForObjects (Transformation|GetActorLocation) (+ (Transformation|GetActorLocation _returnvalue) (Math|Vector|MakeVector 0.0 0.0 (Variables|/Script/Engine.Pawn|GetBaseEyeHeight _returnvalue))) (Utilities|Array|MakeArray "ObjectTypeQuery1" "ObjectTypeQuery2" "ObjectTypeQuery3" "ObjectTypeQuery5" "ObjectTypeQuery6") false (Utilities|Array|MakeArray _returnvalue) "None"))
        (if (not _returnvalue_7)
          (bind _asstab_template (Utilities|Casting|CastToStabTemplate _returnvalue_3)
            (:then
              (Variables|Default|SetTarget (+ (* (Variables|/Game/STAB/Blueprints/Abstract/StabTemplate.StabTemplate_C|GetPerceivedVelocity _asstab_template) _returnvalue_6) _returnvalue_4)))
            (:CastFailed
              (Variables|Default|SetTarget (+ _returnvalue_4 (* (Transformation|GetVelocity _returnvalue_3) _returnvalue_6)))))
          (if (<= (Math|Vector|Distance(Vector) (Variables|Default|GetTarget) (Transformation|GetActorLocation)) (/ (Variables|Default|GetDetectionRange) 3.0))
            (Variables|Default|SetLaserCooldown (- (Variables|Default|GetLaserCooldown) DeltaSeconds))
            (Transformation|SetActorRotation (Math|Interpolation|RInterpTo (Transformation|GetActorRotation) (Math|Rotator|FindLookatRotation (Transformation|GetActorLocation) (Variables|Default|GetTarget)) DeltaSeconds 5.0))
            (if (<= (Variables|Default|GetLaserCooldown) 0.0)
              (Variables|Default|SetLaserCooldown 2.0)
              (bind _returnvalue_8 (Game|SpawnActorfromClass "/Game/STAB/Blueprints/Generated/LaserBolt.LaserBolt_C" (Math|Transform|MakeTransform (+ (* (Math|Vector|GetForwardVector _returnvalue_2) 5e+01) (Transformation|GetActorLocation)) _returnvalue_2 "1,1,1") "AlwaysSpawn" 0 0))
              (Variables|/Game/STAB/Blueprints/Generated/LaserBolt.LaserBolt_C|SetColor _returnvalue_8 (Variables|Default|GetColor))
              (Variables|/Game/STAB/Blueprints/Generated/LaserBolt.LaserBolt_C|SetShooter _returnvalue_8 self))
            (else
              (Transformation|SetWorldRotation _buggy (Math|Interpolation|RInterpTo (Transformation|GetWorldRotation _buggy) (Math|Rotator|MakeRotator 0.0 0.0 (+ (.yaw (Math|Rotator|FindLookatRotation (Transformation|GetWorldLocation _buggy) (Variables|Default|GetTarget))) -9e+01)) DeltaSeconds 1.0) false false)
              (Physics|AddForce _buggy (* (Math|Vector|GetRightVector _buggy) 1e+03) "None" true))))))))

(fn ConstructionScript
  (Rendering|Material|SetVectorParameterValueonMaterials (Variables|Default|GetStaticMesh) "Color" (Variables|Default|GetColor)))

(fn Hurt
  (params (Damage :type Float%20%28single-precision%29) (DamageType :type Damage%20Type%20Object%20Reference) (InstigatedBy :type Controller%20Object%20Reference) (DamageCauser :type Actor%20Object%20Reference)))

(fn DropPickup
  (params (Player :type Stab%20Template%20Object%20Reference))
  (bind _primarycollision (Variables|Default|GetPrimaryCollision))
  (bind _dropped (|CallParentFunction Player))
  (if _dropped
    (return true)
    (elif (Math|Random|RandomBoolwithWeight 0.2)
      (bind _returnvalue (Game|SpawnActorfromClass "/Game/STAB/Blueprints/Players/HackableDrone.HackableDrone_C" (Transformation|GetActorTransform) "AlwaysSpawn" 0 0))
      (Physics|SetPhysicsLinearVelocity (Variables|/Game/STAB/Blueprints/Players/HackableDrone.HackableDrone_C|GetPrimaryCollision _returnvalue) (Transformation|GetComponentVelocity _primarycollision) false "None")
      (Class|PrimitiveComponent|SetPhysicsAngularVelocityinDegrees (Variables|/Game/STAB/Blueprints/Players/HackableDrone.HackableDrone_C|GetPrimaryCollision _returnvalue) (Physics|GetPhysicsAngularVelocityinDegrees _primarycollision "None") false "None")
      (return true))))

(fn ClassTick
  (params (DeltaSeconds :type Float%20%28single-precision%29)))