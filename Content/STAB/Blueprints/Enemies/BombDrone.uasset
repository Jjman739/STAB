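; BombDrone is a kamikaze enemy that homes in on the player and explodes.
; When the player is in range with clear line of sight, Tick smoothly turns it toward a distance-scaled, velocity-led intercept point and applies forward force.
; Hitting the player or taking any damage calls Kaboom, which spawns an explosion, destroys the drone and deals radial damage.
; Damage also credits the attacker, and the construction script tints the mesh.
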(event EventTick
  (params (DeltaSeconds :type Float%20%28single-precision%29))
  (bind _returnvalue (Game|Player|GetPlayerPawn 0))
  (bind _returnvalue_2 (Game|Player|GetPlayerPawn 0))
  (bind _returnvalue_3 (Transformation|GetActorLocation _returnvalue_2))
  (bind _returnvalue_4 (Transformation|GetDistanceTo _returnvalue_2))
  (bind _returnvalue_5 (* _returnvalue_4 0.0004))
  (if (<= (Transformation|GetDistanceTo _returnvalue) (Variables|Default|GetDetectionRange))
    (bind _returnvalue_6 (Collision|LineTraceForObjects (Transformation|GetActorLocation) (+ (Transformation|GetActorLocation _returnvalue) (Math|Vector|MakeVector 0.0 0.0 (Variables|/Script/Engine.Pawn|GetBaseEyeHeight _returnvalue))) (Utilities|Array|MakeArray "ObjectTypeQuery1" "ObjectTypeQuery2" "ObjectTypeQuery3" "ObjectTypeQuery5" "ObjectTypeQuery6") false (Utilities|Array|MakeArray _returnvalue) "None"))
    (if (not _returnvalue_6)
      (bind _asstab_template (Utilities|Casting|CastToStabTemplate _returnvalue_2)
        (:then
          (Variables|Default|SetTarget (+ (* (Variables|/Game/STAB/Blueprints/Abstract/StabTemplate.StabTemplate_C|GetPerceivedVelocity _asstab_template) _returnvalue_5) _returnvalue_3)))
        (:CastFailed
          (Variables|Default|SetTarget (+ _returnvalue_3 (* (Transformation|GetVelocity _returnvalue_2) _returnvalue_5)))))
      (Transformation|SetActorRotation (Math|Interpolation|RInterpTo (Transformation|GetActorRotation) (Math|Rotator|FindLookatRotation (Transformation|GetActorLocation) (Variables|Default|GetTarget)) DeltaSeconds 1e+01))
      (Physics|AddForce (Variables|Default|GetPrimaryCollision) (* (Transformation|GetActorForwardVector) 1e+03) "None" true))))

(event Collision|EventHit
  (params (MyComp :type Primitive%20Component%20Object%20Reference) (Other :type Actor%20Object%20Reference) (OtherComp :type Primitive%20Component%20Object%20Reference) (bSelfMoved :type Boolean) (HitLocation :type Vector :default "0, 0, 0") (HitNormal :type Vector :default "0, 0, 0") (NormalImpulse :type Vector :default "0, 0, 0") (Hit :type Hit%20Result%20Structure%20%28by%20ref%29))
  (if (== Other (Game|Player|GetPlayerPawn 0))
    (CallFunction|Kaboom)))

(event Game|Damage|EventAnyDamage
  (params (Damage :type Float%20%28single-precision%29) (DamageType :type Damage%20Type%20Object%20Reference) (InstigatedBy :type Controller%20Object%20Reference) (DamageCauser :type Actor%20Object%20Reference))
  (CallFunction|GiveHurtCredit DamageCauser (Transformation|GetActorLocation))
  (CallFunction|Kaboom))

(fn ConstructionScript
  (Rendering|Material|SetVectorParameterValueonMaterials (Variables|Default|GetStaticMesh) "Color" (Variables|Default|GetColor)))

(fn Kaboom
  (bind _returnvalue (Transformation|GetActorLocation))
  (bind _self self)
  (Effects|SpawnEmitteratLocation "/Game/STAB/Particles/BombDroneExplosion.BombDroneExplosion" _returnvalue)
  (Actor|DestroyActor)
  (Game|Damage|ApplyRadialDamage 1.0 _returnvalue 3e+02 "/Script/Engine.DamageType" (Utilities|Array|MakeArray _self) _self 0 true "ECC_Visibility"))