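; BasicDrone_AlwaysDrop is an enemy drone variant that always drops a HackableDrone as its pickup.
; Its DropPickup override spawns the HackableDrone at the drone's transform regardless of collision and always returns true, leaving the parent's drop logic unused.
; The new drone inherits the linear and angular velocity of the original's PrimaryCollision, so its motion carries over.
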(event EventBeginPlay)

(event Collision|EventActorBeginOverlap
  (params (OtherActor :type Actor%20Object%20Reference)))

(event EventTick
  (params (DeltaSeconds :type Float%20%28single-precision%29))
  (|CallParentFunction DeltaSeconds) ; This node is disabled and will not be called.\nDrag off pins to build functionality.
)

(fn ConstructionScript
  (|CallParentFunction))

(fn DropPickup
  (params (Player :type Stab%20Template%20Object%20Reference))
  (bind _primarycollision (Variables|Default|GetPrimaryCollision))
  (bind _returnvalue (Game|SpawnActorfromClass "/Game/STAB/Blueprints/Players/HackableDrone.HackableDrone_C" (Transformation|GetActorTransform) "AlwaysSpawn" 0 0))
  (Physics|SetPhysicsLinearVelocity (Variables|/Game/STAB/Blueprints/Players/HackableDrone.HackableDrone_C|GetPrimaryCollision _returnvalue) (Transformation|GetComponentVelocity _primarycollision) false "None")
  (Class|PrimitiveComponent|SetPhysicsAngularVelocityinDegrees (Variables|/Game/STAB/Blueprints/Players/HackableDrone.HackableDrone_C|GetPrimaryCollision _returnvalue) (Physics|GetPhysicsAngularVelocityinDegrees _primarycollision "None") false "None")
  (return true))