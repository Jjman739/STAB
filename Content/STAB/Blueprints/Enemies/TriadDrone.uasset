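; TriadDrone is a three-cannon flying enemy that hunts the player within detection range and line of sight.
; Tick turns it toward a velocity-led aim point, thrusting closer or, within half range, firing lasers from each cannon in turn, slower as HP drops.
; Point hits destroy the struck cannon and radial damage up to two random ones, each costing HP.
; DropPickup can fall back to spawning a HackableDrone that inherits its momentum.
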(event Game|Damage|EventPointDamage
  (params (Damage :type Float%20%28single-precision%29) (DamageType :type Damage%20Type%20Object%20Reference) (HitLocation :type Vector :default "0, 0, 0") (HitNormal :type Vector :default "0, 0, 0") (HitComponent :type Primitive%20Component%20Object%20Reference) (BoneName :type Name :default "None") (ShotFromDirection :type Vector :default "0, 0, 0") (InstigatedBy :type Controller%20Object%20Reference) (DamageCauser :type Actor%20Object%20Reference) (HitInfo :type Hit%20Result%20Structure%20%28by%20ref%29))
  (bind _cannons (Variables|Default|GetCannons))
  (bind _returnvalue (Utilities|Array|FindItem _cannons HitComponent))
  (if (!= _returnvalue -1)
    (CallFunction|DestroyCannon _returnvalue DamageCauser)))

(event EventTick
  (params (DeltaSeconds :type Float%20%28single-precision%29))
  (bind _returnvalue (Game|Player|GetPlayerPawn 0))
  (bind _returnvalue_2 (Game|Player|GetPlayerPawn 0))
  (bind _returnvalue_3 (Transformation|GetActorRotation))
  (bind _cannons (Variables|Default|GetCannons))
  (bind _returnvalue_4 (Utilities|Array|Length _cannons))
  (bind _returnvalue_5 (Transformation|GetActorLocation _returnvalue_2))
  (bind _returnvalue_6 (Transformation|GetDistanceTo _returnvalue_2))
  (bind _returnvalue_7 (* _returnvalue_6 0.0004))
  (Utilities|FlowControl|Sequence
    (:then_0
      (if (<= (Transformation|GetDistanceTo _returnvalue) (Variables|Default|GetDetectionRange))
        (bind _returnvalue_8 (Collision|LineTraceForObjects (Transformation|GetActorLocation) (+ (Transformation|GetActorLocation _returnvalue) (Math|Vector|MakeVector 0.0 0.0 (Variables|/Script/Engine.Pawn|GetBaseEyeHeight _returnvalue))) (Utilities|Array|MakeArray "ObjectTypeQuery1" "ObjectTypeQuery2" "ObjectTypeQuery3" "ObjectTypeQuery5" "ObjectTypeQuery6") false (Utilities|Array|MakeArray _returnvalue) "None"))
        (if (not _returnvalue_8)
          (bind _asstab_template (Utilities|Casting|CastToStabTemplate _returnvalue_2)
            (:then
              (Variables|Default|SetTarget (+ (* (Variables|/Game/STAB/Blueprints/Abstract/StabTemplate.StabTemplate_C|GetPerceivedVelocity _asstab_template) _returnvalue_7) _returnvalue_5)))
            (:CastFailed
              (Variables|Default|SetTarget (+ _returnvalue_5 (* (Transformation|GetVelocity _returnvalue_2) _returnvalue_7)))))
          (Transformation|SetActorRotation (Math|Interpolation|RInterpTo (Transformation|GetActorRotation) (Math|Rotator|FindLookatRotation (Transformation|GetActorLocation) (Variables|Default|GetTarget)) DeltaSeconds 5.0))
          (bind _output_get (Variables|Default|SetLaserCooldown (- (Variables|Default|GetLaserCooldown) DeltaSeconds)))
          (if (<= (Math|Vector|Distance(Vector) (Variables|Default|GetTarget) (Transformation|GetActorLocation)) (/ (Variables|Default|GetDetectionRange) 2.0))
            (if (<= _output_get 0.0)
              (if (< (Variables|Default|GetCannonIndex) _returnvalue_4)
                (Utilities|FlowControl|Sequence
                  (:then_0
                    (Variables|Default|SetLaserCooldown (/ 2.0 (Math|Conversions|ToFloat(Integer) (Variables|Default|GetHP))))
                    (bind _returnvalue_9 (Game|SpawnActorfromClass "/Game/STAB/Blueprints/Generated/LaserBolt.LaserBolt_C" (Math|Transform|MakeTransform (+ (* (Math|Vector|GetForwardVector _returnvalue_3) 5e+01) (Transformation|GetWorldLocation (Utilities|Array|Get(acopy) _cannons (Variables|Default|GetCannonIndex)))) _returnvalue_3 "1,1,1") "AlwaysSpawn" 0 0))
                    (Variables|/Game/STAB/Blueprints/Generated/LaserBolt.LaserBolt_C|SetColor _returnvalue_9 (Variables|Default|GetColor))
                    (Variables|/Game/STAB/Blueprints/Generated/LaserBolt.LaserBolt_C|SetShooter _returnvalue_9 self))
                  (:then_1
                    (if (< (+ (Variables|Default|GetCannonIndex) 1) _returnvalue_4) :!label _label
                      (Variables|Default|SetCannonIndex (+ (Variables|Default|GetCannonIndex) 1))
                      (else
                        (Variables|Default|SetCannonIndex 0)))))
                (else
                  (goto _label))))
            (else
              (Physics|AddForce (Variables|Default|GetPrimaryCollision) (* (Transformation|GetActorForwardVector) 5e+02) "None" true))))))
    (:then_1
      (CallFunction|ClassTick DeltaSeconds))))

(event EventBeginPlay
  (Variables|Default|SetCannons (Utilities|Array|MakeArray (Variables|Default|GetLaserCannonExtension1) (Variables|Default|GetLaserCannonExtension2) (Variables|Default|GetLaserCannonExtension3))))

(event Game|Damage|EventRadialDamage
  (params (DamageReceived :type Float%20%28single-precision%29) (DamageType :type Damage%20Type%20Object%20Reference) (Origin :type Vector :default "0, 0, 0") (HitInfo :type Hit%20Result%20Structure%20%28by%20ref%29) (InstigatedBy :type Controller%20Object%20Reference) (DamageCauser :type Actor%20Object%20Reference))
  (CallFunction|DestroyCannon (.OutIndex (Utilities|Array|Random (Variables|Default|GetCannons))) DamageCauser)
  (if (Utilities|IsValid self)
    (CallFunction|DestroyCannon (.OutIndex (Utilities|Array|Random (Variables|Default|GetCannons))) DamageCauser)))

(fn ConstructionScript
  (Rendering|Material|SetVectorParameterValueonMaterials (Variables|Default|GetStaticMesh) "Color" (Variables|Default|GetColor)))

(fn Hurt
  (params (Damage :type Float%20%28single-precision%29) (DamageType :type Damage%20Type%20Object%20Reference) (InstigatedBy :type Controller%20Object%20Reference) (DamageCauser :type Actor%20Object%20Reference)))

(fn DropPickup
  (params (Player :type Stab%20Template%20Object%20Reference))
  (bind _primarycollision (Variables|Default|GetPrimaryCollision))
  (bind _dropped (|CallParentFunction Player))
  (if _dropped
    (return true)
    (elif (Math|Random|RandomBoolwithWeight 0.2)
      (bind _returnvalue (Game|SpawnActorfromClass "/Game/STAB/Blueprints/Players/HackableDrone.HackableDrone_C" (Transformation|GetActorTransform) "AlwaysSpawn" 0 0))
      (Physics|SetPhysicsLinearVelocity (Variables|/Game/STAB/Blueprints/Players/HackableDrone.HackableDrone_C|GetPrimaryCollision _returnvalue) (Transformation|GetComponentVelocity _primarycollision) false "None")
      (Class|PrimitiveComponent|SetPhysicsAngularVelocityinDegrees (Variables|/Game/STAB/Blueprints/Players/HackableDrone.HackableDrone_C|GetPrimaryCollision _returnvalue) (Physics|GetPhysicsAngularVelocityinDegrees _primarycollision "None") false "None")
      (return true))))

(fn ClassTick
  (params (DeltaSeconds :type Float%20%28single-precision%29)))

(fn DestroyCannon
  (params (CannonIndex :type Integer) (Attacker :type Actor%20Object%20Reference))
  (bind _returnvalue (Transformation|GetActorLocation))
  (bind _cannons (Variables|Default|GetCannons))
  (bind _output_get (LocalVariables|SetCannon (Utilities|Array|Get(acopy) _cannons CannonIndex)))
  (Utilities|Array|RemoveItem _cannons _output_get)
  (Effects|SpawnEmitteratLocation "/Game/STAB/Particles/Explosion.Explosion" (Transformation|GetWorldLocation _output_get) "0, 0, 0" "0.650000,0.650000,0.650000")
  (for _array_element (Components|GetChildrenComponents _output_get false)
    (Components|DestroyComponent _array_element))
  (bind _output_get_2 (Variables|Default|SetHP (- (Variables|Default|GetHP) 1)))
  (if (<= _output_get_2 0)
    (CallFunction|GiveKillCredit Attacker _returnvalue)
    (Effects|SpawnEmitteratLocation "/Game/STAB/Particles/Explosion.Explosion" _returnvalue)
    (Actor|DestroyActor)
    (else
      (CallFunction|GiveHurtCredit Attacker (Transformation|GetWorldLocation _output_get))
      (Components|DestroyComponent _output_get))))