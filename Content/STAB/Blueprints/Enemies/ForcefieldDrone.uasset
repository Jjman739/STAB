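; Forcefield drone enemy that loses at least one HP per accepted hit, with a short invulnerability window counted down in ClassTick.
; HP drives the forcefield sphere's state: it shows a damaged material on non-lethal hits and hides at one HP.
; Hits credit the attacker, and zero HP spawns an explosion, credits the kill and destroys the drone.
; The construction script tints the forcefield with the drone's Color.
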(event Game|Damage|EventAnyDamage
  (params (Damage :type Float%20%28single-precision%29) (DamageType :type Damage%20Type%20Object%20Reference) (InstigatedBy :type Controller%20Object%20Reference) (DamageCauser :type Actor%20Object%20Reference))
  (bind _returnvalue (Transformation|GetActorLocation))
  (bind _forcefieldsphere (Variables|Default|GetForcefieldSphere))
  (if (<= (Variables|Default|GetiFrames) 0.0)
    (Variables|Default|SetiFrames 0.7)
    (bind _output_get (Variables|Default|SetHP (Math|Integer|Clamp(Integer) (- (Variables|Default|GetHP) (Math|Float|Floor Damage)) 0 (- (Variables|Default|GetHP) 1))))
    (switch int _output_get
      (:Default
        (Rendering|Material|SetScalarParameterValueonMaterials _forcefieldsphere "Damaged" 1.0 :!label _label)
        (CallFunction|GiveHurtCredit DamageCauser (Transformation|GetActorLocation) :!label _label_2))
      (:0
        (Effects|SpawnEmitteratLocation "/Game/STAB/Particles/Explosion.Explosion" _returnvalue)
        (CallFunction|GiveKillCredit DamageCauser _returnvalue)
        (Actor|DestroyActor))
      (:1
        (Rendering|SetVisibility _forcefieldsphere false false)
        (goto _label_2))
      (:2
        (goto _label)))
    (else
      (Variables|Default|SetiFrames (- (Variables|Default|GetiFrames) 0.0)))))

(fn ConstructionScript
  (|CallParentFunction)
  (Rendering|Material|SetVectorParameterValueonMaterials (Variables|Default|GetForcefieldSphere) "Color" (Variables|Default|GetColor)))

(fn ClassTick
  (params (DeltaSeconds :type Float%20%28single-precision%29))
  (Variables|Default|SetiFrames (- (Variables|Default|GetiFrames) DeltaSeconds)))