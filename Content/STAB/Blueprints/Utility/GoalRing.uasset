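; GoalRing is a slowly spinning goal actor that ends a run with a score review and collects retrieved drones.
; Tick yaws its scene component at a constant rate.
; Overlap by a StabTemplate actor adds a ScoreReview widget to the viewport.
; An overlapping HackableDrone has NoKaboom set before it is destroyed, and the Scorekeeper's EnemiesRetrieved count goes up.
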(event Collision|EventActorBeginOverlap
  (params (OtherActor :type Actor%20Object%20Reference))
  (Utilities|Casting|CastToStabTemplate OtherActor
    (:then
      (bind _returnvalue (UserInterface|CreateWidget "/Game/STAB/UI/ScoreReview/ScoreReview.ScoreReview_C"))
      (UserInterface|Viewport|AddtoViewport _returnvalue 0))
    (:CastFailed
      (bind _ashackable_drone (Utilities|Casting|CastToHackableDrone OtherActor))
      (Variables|/Game/STAB/Blueprints/Players/HackableDrone.HackableDrone_C|SetNoKaboom _ashackable_drone true)
      (Actor|DestroyActor _ashackable_drone)
      (Math|Integer|IncrementInt (Variables|/Game/STAB/Blueprints/Utility/Scorekeeper.Scorekeeper_C|GetEnemiesRetrieved (Variables|Default|GetScorekeeper))))))

(event EventTick
  (params (DeltaSeconds :type Float%20%28single-precision%29))
  (Transformation|AddRelativeRotation (Variables|Default|GetScene) (Math|Rotator|MakeRotator 0.0 0.0 (* DeltaSeconds 1e+01)) false false))

(fn ConstructionScript)