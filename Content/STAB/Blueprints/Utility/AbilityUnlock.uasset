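; World pickup that permanently records an ability as unlocked in the game instance when the player touches it.
; The construction script sets sprite and spotlight color from the AbilityType class defaults, and the sprite spins on Tick.
; Overlap closes open ability menus, shows an InfoBox and hides the unlock.
; If already unlocked at BeginPlay, it spawns a permanent AbilityPickup in its place and hides itself.
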(event EventTick
  (params (DeltaSeconds :type Float%20%28single-precision%29))
  (Transformation|AddWorldRotation (Variables|Default|GetPaperSprite) (Math|Rotator|MakeRotator 0.0 0.0 (* DeltaSeconds 5e+01)) false false))

(event Collision|EventActorBeginOverlap
  (params (OtherActor :type Actor%20Object%20Reference))
  (if (== OtherActor (Game|Player|GetPlayerPawn 0))
    (Utilities|Casting|CastToStabTemplate OtherActor)
    (bind _asstab_game_instance (Utilities|Casting|CastToStabGameInstance (Game|GetGameInstance)))
    (Utilities|Map|Add (Variables|/Game/STAB/Blueprints/Abstract/StabGameInstance.StabGameInstance_C|GetAbilitiesUnlocked _asstab_game_instance) (.TechnicalName (Utilities|GetClassDefaults (Variables|Default|GetAbilityType))) true)
    (bind _foundwidgets (Widget|GetAllWidgetsOfClass "/Game/STAB/UI/AbilityMenu.AbilityMenu_C" true))
    (if (== (Utilities|Array|Length _foundwidgets) 0)
      _
      (else
        (for _array_element _foundwidgets
          (Default|CloseMenu _array_element))))
    (bind _returnvalue (UserInterface|CreateWidget "/Game/STAB/UI/InfoBox.InfoBox_C"))
    (Variables|/Game/STAB/UI/InfoBox.InfoBox_C|SetUnlockType _returnvalue (Variables|Default|GetAbilityType))
    (UserInterface|Viewport|AddtoViewport _returnvalue 0)
    (Components|DestroyComponent (Variables|Default|GetSpotLight))
    (Rendering|SetVisibility (Variables|Default|GetPaperSprite) false false)))

(event EventBeginPlay
  (bind _asstab_game_instance (Utilities|Casting|CastToStabGameInstance (Game|GetGameInstance)))
  (if (.Value (Utilities|Map|Find (Variables|/Game/STAB/Blueprints/Abstract/StabGameInstance.StabGameInstance_C|GetAbilitiesUnlocked _asstab_game_instance) (.TechnicalName (Utilities|GetClassDefaults (Variables|Default|GetAbilityType)))))
    (bind _returnvalue (Game|SpawnActorfromClass "/Game/STAB/Blueprints/Utility/AbilityPickup.AbilityPickup_C" (Math|Transform|MakeTransform (Transformation|GetWorldLocation (Variables|Default|GetPaperSprite)) "0, 0, 0" "1,1,1") "Undefined" 0 0))
    (Default|SetAbility _returnvalue (Variables|Default|GetAbilityType))
    (Variables|/Game/STAB/Blueprints/Abstract/Pickup.Pickup_C|SetPermanent _returnvalue true)
    (Actor|SetLifeSpan _returnvalue 0.0)
    (Components|DestroyComponent (Variables|Default|GetSpotLight))
    (Rendering|SetVisibility (Variables|Default|GetPaperSprite) false false)))

(fn ConstructionScript
  (bind _abilitytype (Variables|Default|GetAbilityType))
  (bind (_sprite _color) (Utilities|GetClassDefaults _abilitytype))
  (Rendering|Components|Sprite|SetSprite (Variables|Default|GetPaperSprite) _sprite)
  (Rendering|Components|Light|SetLightColor (Variables|Default|GetSpotLight) _color true))