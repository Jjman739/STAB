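; AbilityPickup is a pickup actor that represents one ability class and adds to that ability's count in StabGameInstance.
; Construction and SetAbility read the class defaults to set the sphere color, sprite and technical name.
; PickedUp increments the count keyed by that name, while PermaSpawn destroys the actor if the ability is not unlocked.
; Its overlap and tick events are disabled, and nothing here calls PickedUp or PermaSpawn.
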(event Collision|EventActorBeginOverlap
  (params (OtherActor :type Actor%20Object%20Reference))
  (|CallParentFunction OtherActor) ; This node is disabled and will not be called.\nDrag off pins to build functionality.
)

(event EventTick
  (params (DeltaSeconds :type Float%20%28single-precision%29))
  (|CallParentFunction DeltaSeconds) ; This node is disabled and will not be called.\nDrag off pins to build functionality.
)

(fn ConstructionScript
  (bind _abilitytype (Variables|Default|GetAbilityType))
  (bind (_sprite _color _abilityname _description _technicalname) (Utilities|GetClassDefaults _abilitytype))
  (Rendering|Material|SetVectorParameterValueonMaterials (Variables|Default|GetSphere) "Color" (Math|Conversions|ToVector(LinearColor) _color))
  (Rendering|Components|Sprite|SetSprite (Variables|Default|GetPaperSprite) _sprite)
  (Variables|Default|SetAbilityName _technicalname))

(fn PickedUp
  (params (Player :type Stab%20Template%20Object%20Reference))
  (bind _abilityname (Variables|Default|GetAbilityName))
  (bind _asstab_game_instance (Utilities|Casting|CastToStabGameInstance (Game|GetGameInstance)))
  (Utilities|Map|Add (Variables|/Game/STAB/Blueprints/Abstract/StabGameInstance.StabGameInstance_C|GetAbilityCounts _asstab_game_instance) _abilityname (+ (.Value (Utilities|Map|Find (Variables|/Game/STAB/Blueprints/Abstract/StabGameInstance.StabGameInstance_C|GetAbilityCounts _asstab_game_instance) _abilityname)) 1)))

(fn PermaSpawn
  (bind _asstab_game_instance (Utilities|Casting|CastToStabGameInstance (Game|GetGameInstance)))
  (if (not (.Value (Utilities|Map|Find (Variables|/Game/STAB/Blueprints/Abstract/StabGameInstance.StabGameInstance_C|GetAbilitiesUnlocked _asstab_game_instance) (Variables|Default|GetAbilityName))))
    (Actor|DestroyActor)))

(fn SetAbility
  (params (Ability :type Ability%20Type%20Class%20Reference))
  (bind (_sprite _color _abilityname _description _technicalname) (Utilities|GetClassDefaults Ability))
  (Variables|Default|SetAbilityType Ability)
  (Rendering|Material|SetVectorParameterValueonMaterials (Variables|Default|GetSphere) "Color" (Math|Conversions|ToVector(LinearColor) _color))
  (Rendering|Components|Sprite|SetSprite (Variables|Default|GetPaperSprite) _sprite)
  (Variables|Default|SetAbilityName _technicalname))