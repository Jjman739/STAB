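; Scorekeeper tracks a level's elapsed time and enemy score, then builds the named score breakdown and total.
; It caches the player pawn and game instance on BeginPlay, and GiveEnemyCredit adds flat points regardless of enemy class.
; GetScoring combines remaining HP, unlocked ability counts, enemy score, drone retrievals with diminishing returns, and time bonus.
; The time bonus falls quadratically, capped at full up to MinTime and reaching zero at MaxTime.
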(event EventBeginPlay
  (bind _asstab_template (Utilities|Casting|CastToStabTemplate (Game|Player|GetPlayerPawn 0)))
  (Variables|Default|SetPlayerPawn _asstab_template)
  (bind _asstab_game_instance (Utilities|Casting|CastToStabGameInstance (Game|GetGameInstance)))
  (Variables|Default|SetGameInstance _asstab_game_instance))

(event EventTick
  (params (DeltaSeconds :type Float%20%28single-precision%29))
  (Variables|Default|SetCurrentTimer (+ (Variables|Default|GetCurrentTimer) DeltaSeconds)))

(fn ConstructionScript)

(fn GetTimeScore
  (bind _maxtimebonus (Variables|Default|GetMaxTimeBonus))
  (bind _maxtime (Variables|Default|GetMaxTime))
  (return (Math|Float|Floor (Math|Float|Clamp(Float) (/ (Math|Float|Square (- (Variables|Default|GetMaxTime) (Math|Float|Clamp(Float) (Variables|Default|GetCurrentTimer) 0.0 _maxtime))) (/ (Math|Float|Square (- _maxtime (Variables|Default|GetMinTime))) _maxtimebonus)) 0.0 _maxtimebonus))))

(fn GiveEnemyCredit
  (params (EnemyClass :type Enemy%20Class%20Reference))
  (Variables|Default|SetEnemyScore (+ (Variables|Default|GetEnemyScore) 50)))

(fn GetScoring
  (bind _enemiesretrieved (Variables|Default|GetEnemiesRetrieved))
  (bind _gameinstance (Variables|Default|GetGameInstance))
  (bind _abilitiesunlocked (Variables|/Game/STAB/Blueprints/Abstract/StabGameInstance.StabGameInstance_C|GetAbilitiesUnlocked _gameinstance))
  ;[1 1 1] Remaining HP
  (Utilities|Map|Add (LocalVariables|GetScoreDivisions) "Remaining HP" (* (Variables|/Game/STAB/Blueprints/Abstract/StabTemplate.StabTemplate_C|GetHP (Variables|Default|GetPlayerPawn)) 200))
  ;[1 1 1] Remaining Abilities
  (bind _keys (Utilities|Map|Keys _abilitiesunlocked))
  (for _array_element _keys
    (if (.Value (Utilities|Map|Find _abilitiesunlocked _array_element))
      (LocalVariables|SetAnyAbilities true)
      (LocalVariables|SetAbilityScore (+ (LocalVariables|GetAbilityScore) (* (.Value (Utilities|Map|Find (Variables|/Game/STAB/Blueprints/Abstract/StabGameInstance.StabGameInstance_C|GetAbilityCounts _gameinstance) _array_element)) 100)))))
  (if (LocalVariables|GetAnyAbilities)
    (Utilities|Map|Add (LocalVariables|GetScoreDivisions) "Remaining Abilities" (LocalVariables|GetAbilityScore)))
  ;[1 1 1] Enemies Defeated
  (Utilities|Map|Add (LocalVariables|GetScoreDivisions) "Enemies Defeated" (Variables|Default|GetEnemyScore))
  ;[1 1 1] Drones retrieved
  (if (> _enemiesretrieved 0)
    (for _index (range 1 _enemiesretrieved)
      (LocalVariables|SetRetrieveScore (+ (LocalVariables|GetRetrieveScore) (/ 500 _index))))
    (Utilities|Map|Add (LocalVariables|GetScoreDivisions) "Drones retrieved" (LocalVariables|GetRetrieveScore)))
  ;[1 1 1] Time bonus
  (bind _score (CallFunction|GetTimeScore))
  (Utilities|Map|Add (LocalVariables|GetScoreDivisions) "Time bonus" _score)
  ;[1 1 1] Total
  (bind _values (Utilities|Map|Values (LocalVariables|GetScoreDivisions)))
  (for _array_element_2 _values
    (LocalVariables|SetTotalScore (+ (LocalVariables|GetTotalScore) _array_element_2)))
  (return (Variables|Default|GetLevel%20Name) (LocalVariables|GetScoreDivisions) (LocalVariables|GetTotalScore)))