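; Chemical bomb actor that explodes when it hits something, provided it has a valid Shooter.
; Hit only destroys the actor; the explosion runs in Destroyed, so any destruction with a valid Shooter triggers it.
; The blast spawns a chemical explosion effect and pushes overlapped components with a linear-falloff radial impulse.
; It also applies radial damage that ignores the Shooter but credits them as the damage causer.
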(event Collision|EventHit
  (params (MyComp :type Primitive%20Component%20Object%20Reference) (Other :type Actor%20Object%20Reference) (OtherComp :type Primitive%20Component%20Object%20Reference) (bSelfMoved :type Boolean) (HitLocation :type Vector :default "0, 0, 0") (HitNormal :type Vector :default "0, 0, 0") (NormalImpulse :type Vector :default "0, 0, 0") (Hit :type Hit%20Result%20Structure%20%28by%20ref%29))
  (if (Utilities|IsValid (Variables|Default|GetShooter))
    (Actor|DestroyActor)))

(event EventDestroyed
  (bind _returnvalue (Transformation|GetActorLocation))
  (bind _explosionradius (Variables|Default|GetExplosionRadius))
  (bind _shooter (Variables|Default|GetShooter))
  (if (Utilities|IsValid (Variables|Default|GetShooter))
    (Effects|SpawnEmitteratLocation "/Game/STAB/Particles/ChemicalExplosion.ChemicalExplosion" _returnvalue)
    (bind _outcomponents (Collision|SphereOverlapComponents _returnvalue _explosionradius (Utilities|Array|MakeArray "ObjectTypeQuery2" "ObjectTypeQuery3" "ObjectTypeQuery4" "ObjectTypeQuery5" "ObjectTypeQuery6" "ObjectTypeQuery1")))
    (for _array_element _outcomponents
      (Physics|AddRadialImpulse _array_element _returnvalue (Variables|Default|GetExplosionRadius) 1e+05 "RIF_Linear" false))
    (Game|Damage|ApplyRadialDamage 3.0 _returnvalue _explosionradius "/Script/Engine.DamageType" (Utilities|Array|MakeArray _shooter) _shooter 0 false "ECC_PhysicsBody")))

(fn ConstructionScript)