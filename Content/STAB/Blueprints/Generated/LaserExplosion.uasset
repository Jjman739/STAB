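; LaserExplosion is a colored blast sphere that grows every tick and pushes whatever it reaches.
; Each tick it overlaps components within its scaled radius, then GetCollisionDistance line-traces from the center to confirm a clear hit.
; Physics bodies and characters receive outward inverse-square force, but only physics bodies not owned by the Shooter take point damage.
; The overlap-damage and RadialForce logic is disconnected.
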(event EventTick
  (params (DeltaSeconds :type Float%20%28single-precision%29))
  (bind _sphere (Variables|Default|GetSphere))
  (bind _sphere_2 (Variables|Default|GetSphere))
  (bind _shooter (Variables|Default|GetShooter))
  (bind _returnvalue (Transformation|GetWorldLocation _sphere_2))
  (Transformation|SetWorldScale3D _sphere (+ (Transformation|GetWorldScale _sphere) (* "10.000000,10.000000,10.000000" DeltaSeconds)))
  (Rendering|Material|SetVectorParameterValueonMaterials (Variables|Default|GetSphere) "Color" (Variables|Default|GetColor))
  (bind _outcomponents (Collision|SphereOverlapComponents _returnvalue (* (.x (Transformation|GetWorldScale _sphere_2)) 1e+02) (Utilities|Array|MakeArray "ObjectTypeQuery1" "ObjectTypeQuery2" "ObjectTypeQuery3" "ObjectTypeQuery4" "ObjectTypeQuery5" "ObjectTypeQuery6")))
  (for _array_element _outcomponents
    (if (Utilities|IsValid _array_element)
      (bind (_validhit _distance _hitpoint) (CallFunction|GetCollisionDistance _array_element))
      (if _validhit
        (if (Physics|IsSimulatingPhysics _array_element "None")
          (Physics|AddForce _array_element (* (Math|Vector|GetForwardVector (Math|Rotator|FindLookatRotation _returnvalue _hitpoint)) (/ 1e+07 (Math|Float|Square (Math|Float|Max(Float) _distance 3e+01)))) "None" true)
          (if (!= (Components|GetOwner _array_element) _shooter)
            (Game|Damage|ApplyPointDamage (Components|GetOwner _array_element) 1.0 _hitpoint (Collision|MakeHitResult false false 0.0 _distance _hitpoint "0, 0, 0" "0,0,1" "0,0,1" 0 (Components|GetOwner _array_element) _array_element "None" 0 0 0 "0, 0, 0" "0, 0, 0") 0 _shooter))
          (else
            (bind _ascharacter (Utilities|Casting|CastToCharacter (Components|GetOwner _array_element)))
            (Physics|AddForce (Variables|/Script/Engine.Character|GetCharacterMovement _ascharacter) (* (* (Math|Vector|GetForwardVector (Math|Rotator|FindLookatRotation _returnvalue _hitpoint)) (/ 1e+07 (Math|Float|Square (Math|Float|Max(Float) _distance 3e+01)))) (Variables|/Script/Engine.CharacterMovementComponent|GetMass (Variables|/Script/Engine.Character|GetCharacterMovement _ascharacter))))))))))

(event Collision|EventActorBeginOverlap
  (params (OtherActor :type Actor%20Object%20Reference)))

(fn ConstructionScript)

(fn GetCollisionDistance
  (params (OtherComp :type Primitive%20Component%20Object%20Reference))
  (bind (_outhit _returnvalue) (Class|KismetSystemLibrary|LineTraceSinglebyProfile (Transformation|GetActorLocation) (Transformation|GetWorldLocation OtherComp) (Collision|GetCollisionProfileName OtherComp) false 0 "None" true))
  (if (and _returnvalue (== OtherComp (.HitComponent (Collision|BreakHitResult _outhit))))
    (return true (.Distance (Collision|BreakHitResult _outhit)) (.Location (Collision|BreakHitResult _outhit)))
    (else
      (return false 0.0 "0, 0, 0"))))