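; Physics-driven homing missile actor that deals point damage to anything it hits except its shooter.
; An initial impulse launches it, then Tick pushes it toward the stored target location, or straight ahead without one, and faces it along velocity.
; Each tick a sphere overlap retargets the nearest TargetComponent.
; After a brief arming delay it self-destructs when nearly stopped, spawning an explosion if the shooter is valid.
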(event EventBeginPlay
  (Physics|AddImpulse (Variables|Default|GetHomingMissile) (* (Transformation|GetActorForwardVector) 5e+03) "None" true)
  (Utilities|FlowControl|Delay 0.05)
  (Variables|Default|SetInitialized true))

(event EventTick
  (params (DeltaSeconds :type Float%20%28single-precision%29))
  (bind _returnvalue (Transformation|GetActorLocation))
  (bind _returnvalue_2 (Transformation|GetVelocity))
  (Physics|AddForce (Variables|Default|GetHomingMissile) (Math|Vector|SelectVector (* (Transformation|GetActorForwardVector) 5e+03) (* (Math|Vector|GetForwardVector (Math|Rotator|FindLookatRotation (Transformation|GetActorLocation) (Variables|Default|GetTarget))) 5e+03) (Class|KismetMathLibrary|EqualExactlyVectorVector (Variables|Default|GetTarget) "0, 0, 0")) "None" true)
  (if (Class|KismetMathLibrary|NotEqualExactlyVectorVector _returnvalue_2 "0, 0, 0")
    (Transformation|SetActorRotation (Math|Rotator|FindLookatRotation (Math|Vector|MakeVector 0.0 0.0 0.0) _returnvalue_2)))
  (Rendering|Material|SetVectorParameterValueonMaterials (Variables|Default|GetHomingMissile) "Color" (Variables|Default|GetColor))
  (if (and (Math|Vector|Equal(Vector) _returnvalue_2 "0, 0, 0" 1e+02) (Variables|Default|GetInitialized))
    (Actor|DestroyActor)
    (else
      (bind (_outcomponents _returnvalue_3) (Collision|SphereOverlapComponents _returnvalue 1e+03 (Utilities|Array|MakeArray "ObjectTypeQuery4") "/Game/STAB/Blueprints/Abstract/TargetComponent.TargetComponent_C"))
      (if _returnvalue_3
        (bind _closest (CallFunction|SelectNearest _outcomponents))
        (Variables|Default|SetTarget (Transformation|GetWorldLocation _closest))
        (elif (< (Math|Vector|Distance(Vector) _returnvalue (Variables|Default|GetTarget)) 1e+02)
          (Variables|Default|SetTarget "0, 0, 0"))))))

(event Collision|EventHit
  (params (MyComp :type Primitive%20Component%20Object%20Reference) (Other :type Actor%20Object%20Reference) (OtherComp :type Primitive%20Component%20Object%20Reference) (bSelfMoved :type Boolean) (HitLocation :type Vector :default "0, 0, 0") (HitNormal :type Vector :default "0, 0, 0") (NormalImpulse :type Vector :default "0, 0, 0") (Hit :type Hit%20Result%20Structure%20%28by%20ref%29))
  (bind _shooter (Variables|Default|GetShooter))
  (if (not (== Other _shooter))
    (Game|Damage|ApplyPointDamage Other 1.0 (Transformation|GetActorLocation) Hit 0 _shooter "/Script/Engine.DamageType")))

(event EventDestroyed
  (if (Utilities|IsValid (Variables|Default|GetShooter))
    (Effects|SpawnEmitteratLocation "/Game/STAB/Particles/Explosion.Explosion" (Transformation|GetActorLocation) "0, 0, 0" "0.500000,0.500000,0.500000")))

(fn ConstructionScript)

(fn SelectNearest
  (params (Targets :type Array%20of%20Primitive%20Component%20Object%20References))
  (bind _output_get (LocalVariables|SetCurrentClosest (Utilities|Array|Get(acopy) Targets)))
  (LocalVariables|SetDistance (Math|Vector|Distance(Vector) (Transformation|GetWorldLocation _output_get) (Transformation|GetActorLocation)))
  (for _array_element Targets
    (if (< (Math|Vector|Distance(Vector) (Transformation|GetWorldLocation _array_element) (Transformation|GetActorLocation)) (LocalVariables|GetDistance))
      (LocalVariables|SetCurrentClosest _array_element)
      (LocalVariables|SetDistance (Math|Vector|Distance(Vector) (Transformation|GetWorldLocation _array_element) (Transformation|GetActorLocation)))))
  (return (LocalVariables|GetCurrentClosest)))