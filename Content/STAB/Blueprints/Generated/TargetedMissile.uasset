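; TargetedMissile is a physics-driven homing missile that steers toward TargetEntity, deals point damage on hit and explodes when destroyed.
; BeginPlay launches it forward and tints its material; Tick eases rotation toward the target and applies forward thrust.
; Any damage or hit destroys it, and ending an overlap makes it block Pawns.
; A SelectNearest helper returns the closest of given components, but nothing here calls it.
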(event EventBeginPlay
  (Physics|AddImpulse (Variables|Default|GetHomingMissile) (* (Transformation|GetActorForwardVector) 1e+03) "None" true)
  (Utilities|FlowControl|Delay 0.05)
  (Variables|Default|SetInitialized true)
  (Rendering|Material|SetVectorParameterValueonMaterials (Variables|Default|GetHomingMissile) "Color" (Variables|Default|GetColor)))

(event Collision|EventActorEndOverlap
  (params (OtherActor :type Actor%20Object%20Reference))
  (Collision|SetCollisionResponsetoChannel (Variables|Default|GetHomingMissile) "ECC_Pawn" "ECR_Block"))

(event Game|Damage|EventAnyDamage
  (params (Damage :type Float%20%28single-precision%29) (DamageType :type Damage%20Type%20Object%20Reference) (InstigatedBy :type Controller%20Object%20Reference) (DamageCauser :type Actor%20Object%20Reference))
  (Actor|DestroyActor))

(event EventTick
  (params (DeltaSeconds :type Float%20%28single-precision%29))
  (bind _returnvalue (Transformation|GetActorRotation))
  (Transformation|SetActorRotation (Math|Interpolation|RInterpTo _returnvalue (Math|Rotator|FindLookatRotation (Transformation|GetActorLocation) (Transformation|GetActorLocation (Variables|Default|GetTargetEntity))) DeltaSeconds 5.0))
  (Physics|AddForce (Variables|Default|GetHomingMissile) (* (Math|Vector|GetForwardVector _returnvalue) 2e+03) "None" true))

(event Collision|EventHit
  (params (MyComp :type Primitive%20Component%20Object%20Reference) (Other :type Actor%20Object%20Reference) (OtherComp :type Primitive%20Component%20Object%20Reference) (bSelfMoved :type Boolean) (HitLocation :type Vector :default "0, 0, 0") (HitNormal :type Vector :default "0, 0, 0") (NormalImpulse :type Vector :default "0, 0, 0") (Hit :type Hit%20Result%20Structure%20%28by%20ref%29))
  (Game|Damage|ApplyPointDamage Other 1.0 (Transformation|GetActorLocation) Hit 0 0 "/Script/Engine.DamageType")
  (Actor|DestroyActor))

(event EventDestroyed
  (Effects|SpawnEmitteratLocation "/Game/STAB/Particles/Explosion.Explosion" (Transformation|GetActorLocation) "0, 0, 0" "0.500000,0.500000,0.500000"))

(fn ConstructionScript)

(fn SelectNearest
  (params (Targets :type Array%20of%20Primitive%20Component%20Object%20References))
  (bind _output_get (LocalVariables|SetCurrentClosest (Utilities|Array|Get(acopy) Targets)))
  (LocalVariables|SetDistance (Math|Vector|Distance(Vector) (Transformation|GetWorldLocation _output_get) (Transformation|GetActorLocation)))
  (for _array_element Targets
    (if (< (Math|Vector|Distance(Vector) (Transformation|GetWorldLocation _array_element) (Transformation|GetActorLocation)) (LocalVariables|GetDistance))
      (LocalVariables|SetCurrentClosest _array_element)
      (LocalVariables|SetDistance (Math|Vector|Distance(Vector) (Transformation|GetWorldLocation _array_element) (Transformation|GetActorLocation)))))
  (return (LocalVariables|GetCurrentClosest)))