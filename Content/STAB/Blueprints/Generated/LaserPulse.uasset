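; LaserPulse is a colored laser projectile that plays a sound on spawn and bursts into an explosion when destroyed.
; Its physics capsule launches along the actor's forward vector with random spin, while Tick pushes Color onto the cylinder's materials.
; Any hit destroys it, as do overlaps with actors other than a valid Shooter, ignoring LaserOverlapType actors.
; On destruction it spawns a small LaserExplosion, passing on Color and Shooter.
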(event Collision|EventActorBeginOverlap
  (params (OtherActor :type Actor%20Object%20Reference))
  (bind _shooter (Variables|Default|GetShooter))
  (Utilities|Casting|CastToLaserOverlapType OtherActor
    (:CastFailed
      (if (and (!= OtherActor _shooter) (Utilities|IsValid _shooter))
        (Actor|DestroyActor)))))

(event EventBeginPlay
  (bind _returnvalue (* 1e+03 1.0))
  (bind _returnvalue_2 (* _returnvalue -1.0))
  (Audio|PlaySoundatLocation "/Game/STAB/Sounds/Laser.Laser" (Transformation|GetActorLocation) "0, 0, 0" 1.0 1.0 0.0 0 0 0)
  (Class|PrimitiveComponent|SetPhysicsAngularVelocityinDegrees (Variables|Default|GetCapsule) (Math|Vector|MakeVector (Math|Random|RandomFloatinRange _returnvalue_2 _returnvalue) (Math|Random|RandomFloatinRange _returnvalue_2 _returnvalue) (Math|Random|RandomFloatinRange _returnvalue_2 _returnvalue)) false "None")
  (Physics|SetPhysicsLinearVelocity (Variables|Default|GetCapsule) (* (Transformation|GetActorForwardVector) 3e+03) false "None"))

(event EventTick
  (params (DeltaSeconds :type Float%20%28single-precision%29))
  (Rendering|Material|SetVectorParameterValueonMaterials (Variables|Default|GetCylinder) "Color" (Variables|Default|GetColor)))

(event EventDestroyed
  (bind _returnvalue (Game|SpawnActorfromClass "/Game/STAB/Blueprints/Generated/LaserExplosion.LaserExplosion_C" (Math|Transform|MakeTransform (Transformation|GetWorldLocation (Variables|Default|GetCapsule)) "0, 0, 0" "0.100000,0.100000,0.100000") "AdjustIfPossibleButAlwaysSpawn" 0 0))
  (Variables|/Game/STAB/Blueprints/Generated/LaserExplosion.LaserExplosion_C|SetColor _returnvalue (Variables|Default|GetColor))
  (Variables|/Game/STAB/Blueprints/Generated/LaserExplosion.LaserExplosion_C|SetShooter _returnvalue (Variables|Default|GetShooter)))

(event Collision|EventHit
  (params (MyComp :type Primitive%20Component%20Object%20Reference) (Other :type Actor%20Object%20Reference) (OtherComp :type Primitive%20Component%20Object%20Reference) (bSelfMoved :type Boolean) (HitLocation :type Vector :default "0, 0, 0") (HitNormal :type Vector :default "0, 0, 0") (NormalImpulse :type Vector :default "0, 0, 0") (Hit :type Hit%20Result%20Structure%20%28by%20ref%29))
  (Actor|DestroyActor))

(fn ConstructionScript)