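; LaserBolt is a laser projectile that plays a firing sound on spawn and damages what it strikes.
; Each Tick tints the cylinder with its Color and forces constant physics velocity along the capsule's up vector.
; Overlaps ignore LaserOverlapType and the Shooter, push physics-simulating capsule roots, then damage and destroy; hits apply point damage and destroy.
; Shortly after any overlap ends, the capsule starts blocking Pawns.
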(event Collision|EventActorBeginOverlap
  (params (OtherActor :type Actor%20Object%20Reference))
  (bind _shooter (Variables|Default|GetShooter))
  (bind _capsule (Variables|Default|GetCapsule))
  (Utilities|Casting|CastToLaserOverlapType OtherActor
    (:CastFailed
      (if (and (!= OtherActor _shooter) (Utilities|IsValid _shooter))
        (bind _ascapsule_collision (Utilities|Casting|CastToCapsuleComponent (Variables|/Script/Engine.Actor|GetRootComponent OtherActor))
          (:then
            (if (Physics|IsSimulatingPhysics _ascapsule_collision "None")
              (Physics|AddImpulseatLocation _ascapsule_collision (* (Transformation|GetComponentVelocity _capsule) 1e+01) (Transformation|GetWorldLocation _capsule) "None")))
          (:CastFailed
            _))
        (Actor|DestroyActor)
        (Game|Damage|ApplyDamage OtherActor 1.0 0 (Variables|Default|GetShooter) "/Script/Engine.DamageType")))))

(event EventBeginPlay
  (Audio|PlaySoundatLocation "/Game/STAB/Sounds/Laser.Laser" (Transformation|GetActorLocation) "0, 0, 0" 1.0 1.0 0.0 0 0 0))

(event EventTick
  (params (DeltaSeconds :type Float%20%28single-precision%29))
  (Rendering|Material|SetVectorParameterValueonMaterials (Variables|Default|GetCylinder) "Color" (Variables|Default|GetColor))
  (Physics|SetPhysicsLinearVelocity (Variables|Default|GetCapsule) (* (Math|Vector|GetUpVector (Variables|Default|GetCapsule)) 3e+03) false "None"))

(event Collision|EventActorEndOverlap
  (params (OtherActor :type Actor%20Object%20Reference))
  (Utilities|FlowControl|Delay 0.05)
  (Collision|SetCollisionResponsetoChannel (Variables|Default|GetCapsule) "ECC_Pawn" "ECR_Block"))

(event Collision|EventHit
  (params (MyComp :type Primitive%20Component%20Object%20Reference) (Other :type Actor%20Object%20Reference) (OtherComp :type Primitive%20Component%20Object%20Reference) (bSelfMoved :type Boolean) (HitLocation :type Vector :default "0, 0, 0") (HitNormal :type Vector :default "0, 0, 0") (NormalImpulse :type Vector :default "0, 0, 0") (Hit :type Hit%20Result%20Structure%20%28by%20ref%29))
  (Actor|DestroyActor)
  (Game|Damage|ApplyPointDamage Other 1.0 HitLocation Hit 0 (Variables|Default|GetShooter) "/Script/Engine.DamageType"))

(fn ConstructionScript)