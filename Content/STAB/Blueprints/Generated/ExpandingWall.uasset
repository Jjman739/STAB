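; ExpandingWall is a physics actor that grows into a wall once it comes to rest.
; Tick waits for low velocity, rechecks after a delay, then disables physics and colors the cube.
; It then stretches the cube sideways, then upward to a height cap that Overdriving bypasses.
; Growth advances a material Size parameter that triggers self-destruction past a threshold; Destroyed switches off overdrive on the player's SClassAgent.
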(event EventDestroyed
  (bind _assclass_agent (Utilities|Casting|CastToSClassAgent (Game|Player|GetPlayerPawn 0)))
  (Default|OverdriveToggle _assclass_agent false))

(event EventTick
  (params (DeltaSeconds :type Float%20%28single-precision%29))
  (bind _returnvalue (* DeltaSeconds 2.0))
  (bind _cube (Variables|Default|GetCube))
  (bind _returnvalue_2 (Transformation|GetWorldScale _cube))
  (bind (_x _y _z) (Math|Vector|BreakVector _returnvalue_2))
  (if (Variables|Default|GetActive)
    (if (<= _y 5.0)
      (Transformation|SetWorldScale3D _cube (+ _returnvalue_2 (Math|Vector|MakeVector (* _returnvalue 0.5) (* _returnvalue 3.0) 0.0)))
      (bind _output_get (Variables|Default|SetSize (+ (Variables|Default|GetSize) (/ _returnvalue 15.0)) :!label _label))
      (Rendering|Material|SetScalarParameterValueonMaterials (Variables|Default|GetCube) "Size" _output_get)
      (if (> _output_get 1.2)
        (Actor|DestroyActor))
      (elif (or (<= _z 5.0) (Variables|Default|GetOverdriving))
        (Transformation|SetWorldScale3D _cube (+ _returnvalue_2 (Math|Vector|MakeVector 0.0 0.0 (* _returnvalue 2.0))))
        (goto _label)))
    (else
      (bind _returnvalue_3 (Physics|GetPhysicsLinearVelocity (Variables|Default|GetCube) "None"))
      (if (<= (Math|Vector|VectorLength _returnvalue_3) 0.1)
        (Utilities|FlowControl|Delay 0.2)
        (if (<= (Math|Vector|VectorLength _returnvalue_3) 0.1)
          (Variables|Default|SetActive true)
          (Physics|SetSimulatePhysics (Variables|Default|GetCube) false)
          (Rendering|Material|SetVectorParameterValueonMaterials (Variables|Default|GetCube) "Color" (Variables|Default|GetColor)))))))

(fn ConstructionScript)