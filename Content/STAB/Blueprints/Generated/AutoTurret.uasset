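; Floating auto-turret companion for the player pawn that fires laser bolts at nearby target components.
; Each tick it overlaps a sphere for TargetComponents, and SelectNearest picks the closest with clear line of sight.
; With a target, it turns smoothly and fires on a short cooldown, cycling four muzzles and crediting the player.
; Otherwise, distance-scaled force pulls it toward a point above and along the player's aim.
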(event EventBeginPlay
  (Variables|Default|SetFirePoints (Utilities|Array|MakeArray (Variables|Default|GetFirePoint1) (Variables|Default|GetFirePoint3) (Variables|Default|GetFirePoint2) (Variables|Default|GetFirePoint4)))
  (Variables|Default|SetCommander (Game|Player|GetPlayerPawn 0)))

(event EventTick
  (params (DeltaSeconds :type Float%20%28single-precision%29))
  (bind _returnvalue (Transformation|GetActorRotation))
  (bind _returnvalue_2 (Transformation|GetActorRotation))
  (bind _returnvalue_3 (Transformation|GetActorLocation))
  (bind _commander (Variables|Default|GetCommander))
  (bind _returnvalue_4 (Pawn|GetControlRotation _commander :!class /Script/Engine.Pawn))
  (bind _returnvalue_5 (Transformation|GetActorLocation _commander))
  (bind _returnvalue_6 (Math|Vector|GetForwardVector _returnvalue_4))
  (bind _returnvalue_7 (+ _returnvalue_5 (Math|Vector|MakeVector 0.0 0.0 2e+02)))
  (bind _returnvalue_8 (* _returnvalue_6 2.5e+02))
  (bind _returnvalue_9 (+ _returnvalue_7 _returnvalue_8))
  (bind _returnvalue_10 (Math|Rotator|FindLookatRotation _returnvalue_3 _returnvalue_9))
  (bind _returnvalue_11 (Math|Vector|Distance(Vector) _returnvalue_9 _returnvalue_3))
  (Utilities|FlowControl|Sequence
    (:then_0
      (Variables|Default|SetCooldown (- (Variables|Default|GetCooldown) DeltaSeconds))
      (Rendering|Material|SetVectorParameterValueonMaterials (Variables|Default|GetAutoTurret) "Color" (Variables|Default|GetColor)))
    (:then_1
      (if (Utilities|IsValid (Variables|Default|GetCommander))
        (bind (_outcomponents _returnvalue_12) (Collision|SphereOverlapComponents (Transformation|GetActorLocation) 3e+03 (Utilities|Array|MakeArray "ObjectTypeQuery4") "/Game/STAB/Blueprints/Abstract/TargetComponent.TargetComponent_C"))
        (if _returnvalue_12
          (bind (_closest _found) (CallFunction|SelectNearest _outcomponents))
          (if _found
            (Transformation|SetActorRotation (Math|Interpolation|RInterpTo _returnvalue (Math|Rotator|FindLookatRotation (Transformation|GetActorLocation) (Transformation|GetWorldLocation _closest)) DeltaSeconds 5.0))
            (if (and (Math|Rotator|Equal(Rotator) _returnvalue (Math|Rotator|FindLookatRotation (Transformation|GetActorLocation) (Transformation|GetWorldLocation _closest)) 5.0) (<= (Variables|Default|GetCooldown) 0.0))
              (bind _returnvalue_13 (Game|SpawnActorfromClass "/Game/STAB/Blueprints/Generated/LaserBolt.LaserBolt_C" (Math|Transform|MakeTransform (+ (Transformation|GetWorldLocation (Utilities|Array|Get(acopy) (Variables|Default|GetFirePoints) (Variables|Default|GetFirePointIndex))) (* (Math|Vector|GetForwardVector (Math|Rotator|FindLookatRotation (Transformation|GetWorldLocation (Utilities|Array|Get(acopy) (Variables|Default|GetFirePoints) (Variables|Default|GetFirePointIndex))) (Transformation|GetWorldLocation _closest))) 1e+02)) (Math|Rotator|FindLookatRotation (Transformation|GetWorldLocation (Utilities|Array|Get(acopy) (Variables|Default|GetFirePoints) (Variables|Default|GetFirePointIndex))) (Transformation|GetWorldLocation _closest)) "1,1,1") "AdjustIfPossibleButAlwaysSpawn" 0 0))
              (Variables|/Game/STAB/Blueprints/Generated/LaserBolt.LaserBolt_C|SetShooter _returnvalue_13 (Variables|Default|GetCommander))
              (Variables|/Game/STAB/Blueprints/Generated/LaserBolt.LaserBolt_C|SetColor _returnvalue_13 (Variables|Default|GetColor))
              (Variables|Default|SetCooldown 0.15)
              (bind _result (Math|Integer|IncrementInt (Variables|Default|GetFirePointIndex))
                (:%20%20
                  (if (>= _result 4)
                    (Variables|Default|SetFirePointIndex 0)))))
            (else
              (if (>= _returnvalue_11 2e+02) :!label _label
                (Transformation|SetActorRotation (Math|Interpolation|RInterpTo _returnvalue_2 _returnvalue_10 DeltaSeconds 5.0))
                (else
                  (Transformation|SetActorRotation (Math|Interpolation|RInterpTo _returnvalue_2 _returnvalue_4 DeltaSeconds 5.0))))
              (Physics|AddForce (Variables|Default|GetAutoTurret) (* (Math|Vector|GetForwardVector _returnvalue_10) (* (Math|Float|Sqrt _returnvalue_11) 1e+02)) "None" true)))
          (else
            (goto _label)))))))

(fn ConstructionScript)

(fn SelectNearest
  (params (Targets :type Array%20of%20Primitive%20Component%20Object%20References))
  (bind _returnvalue (Transformation|GetActorLocation))
  (for _array_element Targets
    (if (< (Math|Vector|Distance(Vector) _returnvalue (Transformation|GetWorldLocation _array_element)) (LocalVariables|GetDistance))
      (bind _returnvalue_2 (Collision|LineTraceForObjects _returnvalue (Transformation|GetWorldLocation _array_element) (Utilities|Array|MakeArray "ObjectTypeQuery1" "ObjectTypeQuery2" "ObjectTypeQuery6") false (Utilities|Array|MakeArray (Components|GetOwner _array_element)) "None"))
      (if (not _returnvalue_2)
        (LocalVariables|SetCurrentClosest _array_element)
        (LocalVariables|SetDistance (Math|Vector|Distance(Vector) _returnvalue (Transformation|GetWorldLocation _array_element))))))
  (return (LocalVariables|GetCurrentClosest) (Utilities|IsValid (LocalVariables|GetCurrentClosest))))